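; Ship actor for the end-of-game sequence that sails along a referenced track spline and then hands off to the final mission.
; On BeginPlay it spawns an attenuated horn sound attached to the mesh's Horn socket.
; MoveAlongSpline plays a Duration-scaled timeline that sets ship transform and horn location by spline distance.
; When the timeline finishes, it activates the entrance point and calls LastMission on the player's FirstPersonCharacter.
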(event Custom|MoveAlongSpline
  (Components|Timeline|SetPlayRate (Variables|GetFloat) (/ 1.0 (Variables|Default|GetDuration)))
  (bind _alpha (Timeline|Float Play)
    (:Update
      (Variables|Default|SetAlpha _alpha)
      (Transformation|SetActorLocationAndRotation (Spline|GetLocationatDistanceAlongSpline (Variables|/Game/Cinematic/AirportScene/Airplane/Blueprints/SplineShip.SplineShip_C|GetSpline (Variables|Default|GetTrackReference)) (Math|Float|Lerp 0.0 (Spline|GetSplineLength (Variables|/Game/Cinematic/AirportScene/Airplane/Blueprints/SplineShip.SplineShip_C|GetSpline (Variables|Default|GetTrackReference))) (Variables|Default|GetAlpha)) "World") (Spline|GetRotationatDistanceAlongSpline (Variables|/Game/Cinematic/AirportScene/Airplane/Blueprints/SplineShip.SplineShip_C|GetSpline (Variables|Default|GetTrackReference)) (Math|Float|Lerp 0.0 (Spline|GetSplineLength (Variables|/Game/Cinematic/AirportScene/Airplane/Blueprints/SplineShip.SplineShip_C|GetSpline (Variables|Default|GetTrackReference))) (Variables|Default|GetAlpha)) "World"))
      (Transformation|SetWorldLocation (Variables|Default|GetAudioHorn) (Spline|GetLocationatDistanceAlongSpline (Variables|/Game/Cinematic/AirportScene/Airplane/Blueprints/SplineShip.SplineShip_C|GetSpline (Variables|Default|GetTrackReference)) (Math|Float|Lerp 0.0 (Spline|GetSplineLength (Variables|/Game/Cinematic/AirportScene/Airplane/Blueprints/SplineShip.SplineShip_C|GetSpline (Variables|Default|GetTrackReference))) (Variables|Default|GetAlpha)) "World") false false))
    (:Finished
      (Default|BecameActive (Variables|Default|GetEntracePoint))
      (bind _asfirst_person_character (Utilities|Casting|CastToFirstPersonCharacter (Game|GetPlayerCharacter 0)))
      (Default|LastMission _asfirst_person_character))))

(event EventBeginPlay
  (bind _returnvalue (Audio|SpawnSoundAttached "/Game/FirstPerson/Audio/ShipHorn.ShipHorn" (Variables|Default|GetStaticMesh) "Horn" (Transformation|GetActorLocation) "0, 0, 0" "KeepRelativeOffset" false 0.75 1.0 0.0 "/Game/Cinematic/FinishGame/Ship/Blueprints/ATT_ShipHorn.ATT_ShipHorn" 0 false))
  (Variables|Default|SetAudioHorn _returnvalue))

(event Collision|EventActorBeginOverlap
  (params (OtherActor :type Actor%20Object%20Reference)))

(event EventTick
  (params (DeltaSeconds :type Float%20%28single-precision%29)))

(fn ConstructionScript)