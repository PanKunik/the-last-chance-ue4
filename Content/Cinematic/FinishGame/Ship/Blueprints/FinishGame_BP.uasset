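; FinishGame_BP is the game's ending trigger on the ship, hidden and inactive from BeginPlay until its BecameActive event reveals the mesh and arms it.
; When the player character then overlaps the mesh, it queues survivor and captain dialogue lines and calls FinishedGame on the first-person character's stats widget.
; After a short delay it opens the main menu level.
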(event OnComponentBeginOverlap(StaticMesh)
  (params (OverlappedComponent :type Primitive%20Component%20Object%20Reference) (OtherActor :type Actor%20Object%20Reference) (OtherComp :type Primitive%20Component%20Object%20Reference) (OtherBodyIndex :type Integer) (bFromSweep :type Boolean) (SweepResult :type Hit%20Result%20Structure%20%28by%20ref%29))
  (bind _returnvalue (Game|GetPlayerCharacter 0))
  (if (Variables|Default|GetIsActive?)
    (if (== OtherActor _returnvalue)
      (Class|PlayerStatistics|ShowSentence(Message) _returnvalue "Your voice:" "I survived! " 2.0 false)
      (Class|PlayerStatistics|ShowSentence(Message) _returnvalue "Captain:" "Yes. We are taking you home." 2.0 false)
      (bind _asfirst_person_character (Utilities|Casting|CastToFirstPersonCharacter (Game|GetPlayerCharacter 0)))
      (Default|FinishedGame (Variables|/Game/FirstPersonBP/Blueprints/FirstPersonCharacter.FirstPersonCharacter_C|GetPlayerStatsWidget _asfirst_person_character))
      (Utilities|FlowControl|Delay 5.0)
      (Game|OpenLevel(byName) "MainMenu"))))

(event Custom|BecameActive
  (bind _staticmesh (Variables|Default|GetStaticMesh))
  (Components|Activation|SetActive _staticmesh true true)
  (Rendering|SetVisibility _staticmesh true false)
  (Variables|Default|SetIsActive? true))

(event EventBeginPlay
  (bind _staticmesh (Variables|Default|GetStaticMesh))
  (Components|Activation|SetActive _staticmesh false false)
  (Rendering|SetVisibility _staticmesh false false))

(event Collision|EventActorBeginOverlap
  (params (OtherActor :type Actor%20Object%20Reference)))

(event EventTick
  (params (DeltaSeconds :type Float%20%28single-precision%29)))

(fn ConstructionScript)