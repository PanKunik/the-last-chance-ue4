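; Torch fire actor whose particle effect starts inactive at zero scale and can be switched on or off.
; SetActive toggles the particle system and starts a looping Ignite or Extinguish timer.
; Each timer steps a uniform scale linearly toward full or zero, then clears itself on arrival.
; Neither timer cancels the other, so toggling mid-fade leaves both running.
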(event Custom|SetActive
  (params (IsActive? :type Boolean))
  (bind _output_get (Variables|Default|SetIsActive IsActive?))
  (Components|Activation|SetActive (Variables|Default|GetParticleSystem) _output_get false)
  (if (Variables|Default|GetIsActive)
    (if (not (Utilities|Time|IsTimerActivebyHandle (Variables|Default|GetIgnite_TH)))
      (bind _returnvalue (Utilities|Time|SetTimerbyFunctionName 0 "Ignite" 0.05 true))
      (Variables|Default|SetIgnite_TH _returnvalue))
    (elif (not (Utilities|Time|IsTimerActivebyHandle (Variables|Default|GetExtinguish_TH)))
      (bind _returnvalue_2 (Utilities|Time|SetTimerbyFunctionName 0 "Extinguish" 0.05 true))
      (Variables|Default|SetExtinguish_TH _returnvalue_2))))

(event Custom|Ignite
  (if (< (Variables|Default|GetScale) 1.0)
    (bind _output_get (Variables|Default|SetScale (Math|Interpolation|FInterptoConstant (Variables|Default|GetScale) 1.0 0.05 0.3)))
    (Transformation|SetRelativeScale3D (Variables|Default|GetParticleSystem) (Math|Vector|MakeVector _output_get _output_get _output_get))
    (else
      (Transformation|SetRelativeScale3D (Variables|Default|GetParticleSystem) (Math|Vector|MakeVector (Variables|Default|GetScale) (Variables|Default|GetScale) (Variables|Default|GetScale)))
      (Utilities|Time|ClearandInvalidateTimerbyHandle (Variables|Default|GetIgnite_TH)))))

(event Custom|Extinguish
  (if (> (Variables|Default|GetScale) 0.0)
    (bind _output_get (Variables|Default|SetScale (Math|Interpolation|FInterptoConstant (Variables|Default|GetScale) 0.0 0.05 0.3)))
    (Transformation|SetRelativeScale3D (Variables|Default|GetParticleSystem) (Math|Vector|MakeVector _output_get _output_get _output_get))
    (else
      (Transformation|SetRelativeScale3D (Variables|Default|GetParticleSystem) (Math|Vector|MakeVector (Variables|Default|GetScale) (Variables|Default|GetScale) (Variables|Default|GetScale)))
      (Utilities|Time|ClearandInvalidateTimerbyHandle (Variables|Default|GetExtinguish_TH)))))

(event EventBeginPlay
  (bind _particlesystem (Variables|Default|GetParticleSystem))
  (Variables|Default|SetIsActive false)
  (Components|Activation|SetActive _particlesystem false false)
  (Variables|Default|SetScale 0.0)
  (Transformation|SetRelativeScale3D _particlesystem "0, 0, 0"))

(event Collision|EventActorBeginOverlap
  (params (OtherActor :type Actor%20Object%20Reference)))

(event EventTick
  (params (DeltaSeconds :type Float%20%28single-precision%29)))

(fn ConstructionScript)