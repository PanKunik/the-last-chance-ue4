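; Fire actor that burns for a limited time with a positional flames sound, then removes itself.
; A fast looping timer started on BeginPlay steps RemainingTime toward zero with constant interpolation, using the timer's elapsed time as delta.
; The first step with time left spawns the attenuated sound once and stores it.
; When time runs out, the sound stops and the actor is destroyed.
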(event Custom|FlamesTimer
  (if (> (Variables|Default|GetRemainingTime) 0.0)
    (Variables|Default|SetRemainingTime (Math|Interpolation|FInterptoConstant (Variables|Default|GetRemainingTime) 0.0 (Class|KismetSystemLibrary|GetTimerElapsedTimeHandle (Variables|Default|GetFlamesTimer_TH)) 1.0))
    (Utilities|FlowControl|DoOnce false
      (:Completed
        (bind _returnvalue (Audio|SpawnSoundatLocation "/Game/FirstPerson/Audio/Flames.Flames" (Transformation|GetActorLocation) "0, 0, 0" 1.0 1.0 0.0 "/Game/FirstPerson/Audio/ATT_BigFlames.ATT_BigFlames" 0 false))
        (Variables|Default|SetFlamesSound _returnvalue)))
    (else
      (Audio|Components|Audio|Stop (Variables|Default|GetFlamesSound))
      (Actor|DestroyActor))))

(event EventBeginPlay
  (bind _returnvalue (Utilities|Time|SetTimerbyFunctionName 0 "FlamesTimer" 0.05 true))
  (Variables|Default|SetFlamesTimer_TH _returnvalue))

(event EventTick
  (params (DeltaSeconds :type Float%20%28single-precision%29)))

(fn ConstructionScript)