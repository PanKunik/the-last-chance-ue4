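; BP_OceanWaves is an actor that plays an attenuated ocean wave sound at its location, repeating it with randomised pauses.
; It spawns the audio component on BeginPlay and starts a looping quarter-second timer that polls whether the sound is playing.
; During playback, a DoOnce picks a random delay and re-sets the sound.
; Once playback stops, the DoOnce resets and FInterpToConstant counts the delay down before replaying.
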(event Custom|SoundLoop
  (bind _oceanwaves (Variables|Default|GetOceanWaves))
  (Utilities|IsValid _oceanwaves
    (:Is%20Valid
      (if (Audio|Components|Audio|IsPlaying _oceanwaves)
        (Utilities|FlowControl|DoOnce false :!label _label
          (:Completed
            (Variables|Default|SetDelay (Math|Random|RandomFloatinRange 2.5 7.5))
            (Audio|Components|Audio|SetSound (Variables|Default|GetOceanWaves) "/Game/FirstPerson/Audio/OceanWaves.OceanWaves")))
        (else
          (Utilities|FlowControl|Sequence
            (:then_0
              (goto _label Reset))
            (:then_1
              (bind _output_get (Variables|Default|SetDelay (Math|Interpolation|FInterptoConstant (Variables|Default|GetDelay) 0.0 (Class|KismetSystemLibrary|GetTimerElapsedTimeHandle (Variables|Default|GetNewVar_0)) 1.0)))
              (if (not (> _output_get 0.0))
                (Audio|Components|Audio|Play (Variables|Default|GetOceanWaves) 0.0)))))))))

(event EventBeginPlay
  (bind _returnvalue (Audio|SpawnSoundatLocation "/Game/FirstPerson/Audio/OceanWaves.OceanWaves" (Transformation|GetActorLocation) "0, 0, 0" 1.0 1.0 0.0 "/Game/FirstPerson/Audio/ATT_Waves.ATT_Waves" 0 false))
  (Variables|Default|SetOceanWaves _returnvalue)
  (bind _returnvalue_2 (Utilities|Time|SetTimerbyFunctionName 0 "SoundLoop" 0.25 true))
  (Variables|Default|SetNewVar_0 _returnvalue_2))

(fn ConstructionScript)