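; Ambient bird sound emitter that plays random bird sounds at its location with attenuation, separated by random pauses.
; BeginPlay spawns one persistent audio component and starts a looping timer that polls it through SoundLoop.
; Once per playback, SoundLoop sets a random sound and delay on that component.
; When playback stops, it interpolates the delay down toward zero, then plays again, avoiding Tick logic.
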(event Custom|SoundLoop
  (bind _birdssound (Variables|Default|GetBirdsSound))
  (Utilities|IsValid _birdssound
    (:Is%20Valid
      (if (Audio|Components|Audio|IsPlaying _birdssound)
        (Utilities|FlowControl|DoOnce false :!label _label
          (:Completed
            (Variables|Default|SetDelay (Math|Random|RandomFloatinRange 2.0 2e+01))
            (Audio|Components|Audio|SetSound (Variables|Default|GetBirdsSound) (Utilities|Array|Get(acopy) (Variables|Default|GetSounds) (Math|Random|RandomIntegerinRange 0 (- (Utilities|Array|Length (Variables|Default|GetSounds)) 1))))))
        (else
          (Utilities|FlowControl|Sequence
            (:then_0
              (goto _label Reset))
            (:then_1
              (bind _output_get (Variables|Default|SetDelay (Math|Interpolation|FInterptoConstant (Variables|Default|GetDelay) 0.0 (Class|KismetSystemLibrary|GetTimerElapsedTimeHandle (Variables|Default|GetNewVar_0)) 1.0)))
              (if (not (> _output_get 0.0))
                (Audio|Components|Audio|Play (Variables|Default|GetBirdsSound) 0.0)))))))))

(event EventBeginPlay
  (bind _returnvalue (Audio|SpawnSoundatLocation (Utilities|Array|Get(acopy) (Variables|Default|GetSounds) (Math|Random|RandomIntegerinRange 0 (- (Utilities|Array|Length (Variables|Default|GetSounds)) 1))) (Transformation|GetActorLocation) "0, 0, 0" 1.0 1.0 0.0 "/Game/FirstPerson/Audio/ATT_Birds.ATT_Birds" 0 false))
  (Variables|Default|SetBirdsSound _returnvalue)
  (bind _returnvalue_2 (Utilities|Time|SetTimerbyFunctionName 0 "SoundLoop" 0.25 true))
  (Variables|Default|SetNewVar_0 _returnvalue_2))

(event Collision|EventActorBeginOverlap
  (params (OtherActor :type Actor%20Object%20Reference)))

(event EventTick
  (params (DeltaSeconds :type Float%20%28single-precision%29)))

(fn ConstructionScript)