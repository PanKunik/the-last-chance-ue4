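; Fish actor that swims and wanders on its own, steering around obstacles; despite the "Flocking" name it ignores neighbours.
; A looping timer casts a fan of forward traces; on a hit it probes side, back and vertical directions and turns toward a random free one.
; Player overlap with AttackAvoid boosts speed, easing down after overlap ends.
; Chase and hit-based steering is disconnected, and traces draw debug lines.
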(event OnComponentHit(ObstacleAvoiding)
  (params (HitComponent :type Primitive%20Component%20Object%20Reference) (OtherActor :type Actor%20Object%20Reference) (OtherComp :type Primitive%20Component%20Object%20Reference) (NormalImpulse :type Vector :default "0, 0, 0") (Hit :type Hit%20Result%20Structure%20%28by%20ref%29))
  (Variables|Default|SetHitResult Hit)
  (Variables|States|SetIsAvoidingObstacle true)
  (Variables|States|SetIsSwimmingFree false)
  (if (not (== OtherActor (Game|Player|GetPlayerPawn 0)))
    (Variables|Default|SetRandVec (* (Math|Random|RandomUnitVector) 3.0))))

(event OnComponentBeginOverlap(AttackAvoid)
  (params (OverlappedComponent :type Primitive%20Component%20Object%20Reference) (OtherActor :type Actor%20Object%20Reference) (OtherComp :type Primitive%20Component%20Object%20Reference) (OtherBodyIndex :type Integer) (bFromSweep :type Boolean) (SweepResult :type Hit%20Result%20Structure%20%28by%20ref%29))
  (Variables|States|SetIsChased true)
  (if (== OtherActor (Game|Player|GetPlayerPawn 0))
    (Variables|Default|SetChaseVec (- (Transformation|GetActorLocation) (Transformation|GetActorLocation OtherActor)))
    (Variables|Default|SetSpeed 5e+02)
    (if (Utilities|Time|IsTimerActivebyHandle (Variables|Default|GetFishSpeedDecreaseHandle))
      (Utilities|Time|ClearandInvalidateTimerbyHandle (Variables|Default|GetFishSpeedDecreaseHandle)))))

(event OnComponentEndOverlap(AttackAvoid)
  (params (OverlappedComponent :type Primitive%20Component%20Object%20Reference) (OtherActor :type Actor%20Object%20Reference) (OtherComp :type Primitive%20Component%20Object%20Reference) (OtherBodyIndex :type Integer))
  (if (Utilities|Time|IsTimerActivebyHandle (Variables|Default|GetFishSpeedDecreaseHandle))
    (Utilities|Time|ClearandInvalidateTimerbyHandle (Variables|Default|GetFishSpeedDecreaseHandle)))
  (bind _returnvalue (Utilities|Time|SetTimerbyFunctionName 0 "SlowDown" (Variables|Default|GetTimeTick) true))
  (Variables|Default|SetFishSpeedDecreaseHandle _returnvalue))

(event Custom|Flocking
  (bind _returnvalue (Transformation|GetActorLocation))
  (bind _returnvalue_2 (Transformation|GetActorLocation))
  (bind _returnvalue_3 (Transformation|GetActorLocation))
  (bind _returnvalue_4 (Transformation|GetActorLocation))
  (bind _returnvalue_5 (Transformation|GetActorLocation))
  (bind _returnvalue_6 (Transformation|GetActorLocation))
  (bind _returnvalue_7 (Transformation|GetActorLocation))
  (bind _returnvalue_8 (Transformation|GetActorLocation))
  (bind _returnvalue_9 (Transformation|GetActorLocation))
  (bind _returnvalue_10 (Transformation|GetActorRotation))
  (bind _returnvalue_11 (Transformation|GetActorLocation))
  (bind _returnvalue_12 (Transformation|GetActorLocation))
  (bind _returnvalue_13 (Transformation|GetActorLocation))
  (bind _returnvalue_14 (Transformation|GetActorLocation))
  (bind _returnvalue_15 (Transformation|GetActorLocation))
  (bind _returnvalue_16 (Transformation|GetActorLocation))
  (bind _isdirectiontracefree (Variables|Default|GetIsDirectionTraceFree))
  (bind _isdirectiontracefree_2 (Variables|Default|GetIsDirectionTraceFree))
  (bind _isdirectiontracefree_3 (Variables|Default|GetIsDirectionTraceFree))
  (Utilities|FlowControl|Sequence
    (:then_0
      (bind _returnvalue_17 (Collision|LineTraceByChannel _returnvalue_15 (+ _returnvalue_15 (* (Transformation|GetActorForwardVector) 2e+02)) "TraceTypeQuery1" false 0 (Variables|Default|GetVisibleTrace?)))
      (Utilities|Array|SetArrayElem (Variables|Default|GetWasFrontLinesHit) 0 _returnvalue_17 true)
      (bind _returnvalue_18 (Collision|LineTraceByChannel _returnvalue (+ _returnvalue (Math|Vector|RotateVector (* (Transformation|GetActorForwardVector) 2e+02) "45.000000, 0,0.000000")) "TraceTypeQuery1" false 0 (Variables|Default|GetVisibleTrace?)))
      (Utilities|Array|SetArrayElem (Variables|Default|GetWasFrontLinesHit) 1 _returnvalue_18 true)
      (bind _returnvalue_19 (Collision|LineTraceByChannel _returnvalue_2 (+ _returnvalue_2 (Math|Vector|RotateVector (* (Transformation|GetActorForwardVector) 2e+02) "-45.000000, 0,0.000000")) "TraceTypeQuery1" false 0 (Variables|Default|GetVisibleTrace?)))
      (Utilities|Array|SetArrayElem (Variables|Default|GetWasFrontLinesHit) 2 _returnvalue_19 true)
      (bind _returnvalue_20 (Collision|LineTraceByChannel _returnvalue_3 (+ _returnvalue_3 (Math|Vector|RotateVector (* (Transformation|GetActorForwardVector) 2e+02) "0.000000,45.000000,0.000000")) "TraceTypeQuery1" false 0 (Variables|Default|GetVisibleTrace?)))
      (Utilities|Array|SetArrayElem (Variables|Default|GetWasFrontLinesHit) 3 _returnvalue_20 true)
      (bind _returnvalue_21 (Collision|LineTraceByChannel _returnvalue_4 (+ _returnvalue_4 (Math|Vector|RotateVector (* (Transformation|GetActorForwardVector) 2e+02) "0.000000,-45.000000,0.000000")) "TraceTypeQuery1" false 0 (Variables|Default|GetVisibleTrace?)))
      (Utilities|Array|SetArrayElem (Variables|Default|GetWasFrontLinesHit) 4 _returnvalue_21 true)
      (bind _returnvalue_22 (Collision|LineTraceByChannel _returnvalue_5 (+ _returnvalue_5 (Math|Vector|RotateVector (* (Transformation|GetActorForwardVector) 2e+02) "-45.000000,45.000000,0.000000")) "TraceTypeQuery1" false 0 (Variables|Default|GetVisibleTrace?)))
      (Utilities|Array|SetArrayElem (Variables|Default|GetWasFrontLinesHit) 5 _returnvalue_22 true)
      (bind _returnvalue_23 (Collision|LineTraceByChannel _returnvalue_6 (+ _returnvalue_6 (Math|Vector|RotateVector (* (Transformation|GetActorForwardVector) 2e+02) "-45.000000,-45.000000,0.000000")) "TraceTypeQuery1" false 0 (Variables|Default|GetVisibleTrace?)))
      (Utilities|Array|SetArrayElem (Variables|Default|GetWasFrontLinesHit) 6 _returnvalue_23 true)
      (bind _returnvalue_24 (Collision|LineTraceByChannel _returnvalue_16 (+ _returnvalue_16 (Math|Vector|RotateVector (* (Transformation|GetActorForwardVector) 2e+02) "45.000000,45.000000,0.000000")) "TraceTypeQuery1" false 0 (Variables|Default|GetVisibleTrace?)))
      (Utilities|Array|SetArrayElem (Variables|Default|GetWasFrontLinesHit) 7 _returnvalue_24 true)
      (bind _returnvalue_25 (Collision|LineTraceByChannel _returnvalue_12 (+ _returnvalue_12 (Math|Vector|RotateVector (* (Transformation|GetActorForwardVector) 2e+02) "45.000000,-45.000000,0.000000")) "TraceTypeQuery1" false 0 (Variables|Default|GetVisibleTrace?)))
      (Utilities|Array|SetArrayElem (Variables|Default|GetWasFrontLinesHit) 8 _returnvalue_25 true))
    (:then_1
      (bind _array_element (Utilities|Array|ForEachLoopwithBreak (Variables|Default|GetWasFrontLinesHit) :!label _label)
        (:LoopBody
          (if _array_element
            (Utilities|FlowControl|Sequence
              (:then_0
                (goto _label Break))
              (:then_1
                (if (not (Variables|Default|GetFoundNewTrace))
                  (bind _returnvalue_26 (Collision|LineTraceByChannel _returnvalue_9 (+ _returnvalue_9 (* (Transformation|GetActorRightVector) 2e+02)) "TraceTypeQuery1" false 0 (Variables|Default|GetVisibleTrace?)))
                  (Utilities|Array|SetArrayElem (Variables|Default|GetIsDirectionTraceFree) 0 (not _returnvalue_26) true)
                  (bind _returnvalue_27 (Collision|LineTraceByChannel _returnvalue_11 (+ _returnvalue_11 (* (Transformation|GetActorRightVector) -2e+02)) "TraceTypeQuery1" false 0 (Variables|Default|GetVisibleTrace?)))
                  (Utilities|Array|SetArrayElem (Variables|Default|GetIsDirectionTraceFree) 1 (not _returnvalue_27) true)
                  (bind _returnvalue_28 (Collision|LineTraceByChannel _returnvalue_13 (+ _returnvalue_13 (* (Transformation|GetActorForwardVector) -2e+02)) "TraceTypeQuery1" false 0 (Variables|Default|GetVisibleTrace?)))
                  (Utilities|Array|SetArrayElem (Variables|Default|GetIsDirectionTraceFree) 2 (not _returnvalue_28) true)
                  (bind _returnvalue_29 (Collision|LineTraceByChannel _returnvalue_14 (+ _returnvalue_14 (* (Transformation|GetActorUpVector) 2e+02)) "TraceTypeQuery1" false 0 (Variables|Default|GetVisibleTrace?)))
                  (Utilities|Array|SetArrayElem (Variables|Default|GetIsDirectionTraceFree) 3 (not _returnvalue_29) true)
                  (bind _returnvalue_30 (Collision|LineTraceByChannel _returnvalue_8 (+ _returnvalue_8 (* (Transformation|GetActorUpVector) -2e+02)) "TraceTypeQuery1" false 0 (Variables|Default|GetVisibleTrace?)))
                  (Utilities|Array|SetArrayElem (Variables|Default|GetIsDirectionTraceFree) 4 (not _returnvalue_30) true)
                  (while (not (Variables|Default|GetFoundNewTrace))
                    (bind _output_get (Variables|Default|SetTraceIndex (Math|Random|RandomIntegerinRange 0 4)))
                    (if (Utilities|Array|Get(acopy) (Variables|Default|GetIsDirectionTraceFree) _output_get)
                      (Variables|Default|SetFoundNewTrace true)))
                  (switch int (Variables|Default|GetTraceIndex)
                    (:0
                      (if (Utilities|Array|Get(acopy) _isdirectiontracefree 3)
                        (Variables|Default|SetNewDirectionRotation (Math|Rotator|FindLookatRotation (Transformation|GetActorForwardVector) (Math|Vector|RotateVector (Transformation|GetActorRightVector) "45.000000,0.000000, 0")))
                        (elif (Utilities|Array|Get(acopy) _isdirectiontracefree 4)
                          (Variables|Default|SetNewDirectionRotation (Math|Rotator|FindLookatRotation (Transformation|GetActorForwardVector) (Math|Vector|RotateVector (Transformation|GetActorRightVector) "-45.000000,0.000000, 0")))
                          (else
                            (Variables|Default|SetNewDirectionRotation (Math|Rotator|FindLookatRotation (Transformation|GetActorForwardVector) (Transformation|GetActorRightVector)))))))
                    (:1
                      (if (Utilities|Array|Get(acopy) _isdirectiontracefree_2 3)
                        (Variables|Default|SetNewDirectionRotation (Math|Rotator|FindLookatRotation (Transformation|GetActorForwardVector) (* (Math|Vector|RotateVector (Transformation|GetActorRightVector) "45.000000, 0, 0") -1.0)))
                        (elif (Utilities|Array|Get(acopy) _isdirectiontracefree_2 4)
                          (Variables|Default|SetNewDirectionRotation (Math|Rotator|FindLookatRotation (Transformation|GetActorForwardVector) (* (Math|Vector|RotateVector (Transformation|GetActorRightVector) "-45.000000, 0, 0") -1.0)))
                          (else
                            (Variables|Default|SetNewDirectionRotation (Math|Rotator|FindLookatRotation (Transformation|GetActorForwardVector) (* (Transformation|GetActorRightVector) -1.0)))))))
                    (:2
                      (if (Utilities|Array|Get(acopy) _isdirectiontracefree_3 3)
                        (Variables|Default|SetNewDirectionRotation (Math|Rotator|FindLookatRotation (Transformation|GetActorForwardVector) (* (Math|Vector|RotateVector (Transformation|GetActorForwardVector) "45.000000, 0, 0") -1.0)))
                        (elif (Utilities|Array|Get(acopy) _isdirectiontracefree_3 4)
                          (Variables|Default|SetNewDirectionRotation (Math|Rotator|FindLookatRotation (Transformation|GetActorForwardVector) (* (Math|Vector|RotateVector (Transformation|GetActorForwardVector) "-45.000000, 0, 0") -1.0)))
                          (else
                            (Variables|Default|SetNewDirectionRotation (Math|Rotator|FindLookatRotation (Transformation|GetActorForwardVector) (* (Transformation|GetActorForwardVector) -1.0)))))))
                    (:3
                      (Variables|Default|SetNewDirectionRotation (Math|Rotator|FindLookatRotation (Transformation|GetActorForwardVector) (Transformation|GetActorUpVector))))
                    (:4
                      (Variables|Default|SetNewDirectionRotation (Math|Rotator|FindLookatRotation (Transformation|GetActorForwardVector) (* (Transformation|GetActorUpVector) -1.0))))))))))))
    (:then_2
      (Transformation|SetWorldLocation (Variables|Default|GetFish) (Math|Vector|Lerp(Vector) _returnvalue_7 (+ _returnvalue_7 (* (Transformation|GetActorForwardVector) (Variables|Default|GetSpeed))) (Variables|Default|GetTimeTick)) true false)
      (if (Variables|Default|GetFoundNewTrace)
        (Transformation|SetActorRotation (Class|KismetMathLibrary|RInterptoConstant _returnvalue_10 (Variables|Default|GetNewDirectionRotation) (Variables|Default|GetTimeTick) 3e+02))
        (if (Math|Rotator|Equal(Rotator) (Class|KismetMathLibrary|RInterptoConstant _returnvalue_10 (Variables|Default|GetNewDirectionRotation) (Variables|Default|GetTimeTick) 3e+02) _returnvalue_10 0.1)
          (Variables|Default|SetFoundNewTrace false))
        (else
          (if (<= (Math|Random|RandomInteger 1000) 50)
            (Variables|Default|SetNewDirectionRotation (Math|Rotator|FindLookatRotation (Transformation|GetActorForwardVector) (Math|Random|RandomUnitVector))))
          (Transformation|SetActorRotation (Class|KismetMathLibrary|RInterptoConstant (Transformation|GetActorRotation) (Variables|Default|GetNewDirectionRotation) (Variables|Default|GetTimeTick) 1e+01)))))))

(event Custom|SlowDown
  (bind _output_get (Variables|Default|SetSpeed (Math|Interpolation|FInterptoConstant (Variables|Default|GetSpeed) 2e+02 (Variables|Default|GetTimeTick) 1e+02)))
  (if (== _output_get 2e+02)
    (Variables|States|SetIsChased false)
    (Utilities|Time|ClearandInvalidateTimerbyHandle (Variables|Default|GetFishSpeedDecreaseHandle))))

(event EventBeginPlay
  (Utilities|Time|SetTimerbyFunctionName self "Flocking" (Variables|Default|GetTimeTick) true))

(fn ConstructionScript)