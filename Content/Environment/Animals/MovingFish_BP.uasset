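; Fish actor that, when flagged active, swims continuously along the spline of a referenced track actor.
; On BeginPlay, a Swim timeline with play rate set from Duration drives position and rotation by distance along the spline in world space.
; When the timeline finishes, it restarts from FishStartOffset, so each repeat begins at that offset rather than necessarily at the spline start.
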(event Custom|MoveAlongSpline
  (Components|Timeline|SetPlayRate (Variables|Default|GetSwim) (/ 1.0 (Variables|Default|GetDuration)))
  (Components|Timeline|SetNewTime (Variables|Default|GetSwim) (Variables|Default|GetFishStartOffset))
  (bind _alpha (Timeline|Swim Play)
    (:Update
      (Variables|Default|SetAlpha _alpha)
      (Transformation|SetActorLocationAndRotation (Spline|GetLocationatDistanceAlongSpline (Variables|/Game/Environment/Animals/SplineTrack.SplineTrack_C|GetPathSpline (Variables|Default|GetTrackReference)) (Math|Float|Lerp 0.0 (Spline|GetSplineLength (Variables|/Game/Environment/Animals/SplineTrack.SplineTrack_C|GetPathSpline (Variables|Default|GetTrackReference))) (Variables|Default|GetAlpha)) "World") (Spline|GetRotationatDistanceAlongSpline (Variables|/Game/Environment/Animals/SplineTrack.SplineTrack_C|GetPathSpline (Variables|Default|GetTrackReference)) (Math|Float|Lerp 0.0 (Spline|GetSplineLength (Variables|/Game/Environment/Animals/SplineTrack.SplineTrack_C|GetPathSpline (Variables|Default|GetTrackReference))) (Variables|Default|GetAlpha)) "World")))
    (:Finished
      (CallFunction|MoveAlongSpline))))

(event EventBeginPlay
  (if (Variables|Default|GetActiveFish)
    (CallFunction|MoveAlongSpline)))

(event Collision|EventActorBeginOverlap
  (params (OtherActor :type Actor%20Object%20Reference)))

(event EventTick
  (params (DeltaSeconds :type Float%20%28single-precision%29)))

(fn ConstructionScript)