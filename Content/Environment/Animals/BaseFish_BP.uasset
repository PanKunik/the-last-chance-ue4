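; BaseFish_BP is a base fish actor that wanders on its own, with no awareness of other fish despite its "Flocking" timer.
; One second after BeginPlay, a fast looping timer sweeps the Sphere forward, scaling Speed by the timer's elapsed time.
; Unblocked moves occasionally pick a random heading and ease the actor's rotation toward it.
; Sphere hits snap it to a randomized, reversed pitch and yaw with zero roll.
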(event OnComponentHit(Sphere)
  (params (HitComponent :type Primitive%20Component%20Object%20Reference) (OtherActor :type Actor%20Object%20Reference) (OtherComp :type Primitive%20Component%20Object%20Reference) (NormalImpulse :type Vector :default "0, 0, 0") (Hit :type Hit%20Result%20Structure%20%28by%20ref%29))
  (bind _returnvalue (Math|Random|RandomRotator false))
  (bind _sphere (Variables|Default|GetSphere))
  (bind _returnvalue_2 (Transformation|GetWorldRotation _sphere))
  (bind _returnvalue_3 (* _returnvalue_2 -1))
  (bind _returnvalue_4 (Math|Rotator|CombineRotators _returnvalue_3 _returnvalue))
  (bind (_roll _pitch _yaw) (Math|Rotator|BreakRotator _returnvalue_4))
  (Transformation|SetWorldRotation _sphere (Math|Rotator|MakeRotator 0.0 _pitch _yaw) false false))

(event Custom|FlockingTimer
  (bind _returnvalue (Transformation|GetActorLocation))
  (bind _sphere (Variables|Default|GetSphere))
  (Utilities|IsValid _sphere
    (:Is%20Valid
      (bind _sweephitresult (Transformation|SetWorldLocation _sphere (Math|Vector|Lerp(Vector) _returnvalue (+ _returnvalue (* (Transformation|GetActorForwardVector) (Variables|Default|GetSpeed))) (Class|KismetSystemLibrary|GetTimerElapsedTimeHandle (Variables|Default|GetFlockingTimer_TH))) true false))
      (if (not (.bBlockingHit (Collision|BreakHitResult _sweephitresult)))
        (if (<= (Math|Random|RandomInteger 1000) 50)
          (Variables|Default|SetNewDirectionRotation (Math|Rotator|FindLookatRotation (Transformation|GetActorForwardVector) (Math|Random|RandomUnitVector))))
        (Transformation|SetActorRotation (Class|KismetMathLibrary|RInterptoConstant (Transformation|GetActorRotation) (Variables|Default|GetNewDirectionRotation) 0.05 1e+01))))))

(event EventBeginPlay
  (Utilities|FlowControl|Delay 1.0)
  (bind _returnvalue (Utilities|Time|SetTimerbyFunctionName 0 "FlockingTimer" 0.01 true))
  (Variables|Default|SetFlockingTimer_TH _returnvalue))

(event Collision|EventActorBeginOverlap
  (params (OtherActor :type Actor%20Object%20Reference)))

(fn ConstructionScript)