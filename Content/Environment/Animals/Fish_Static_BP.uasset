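; Fish actor for ambient sea life that swims forward on Tick through a swept move of its Fish component.
; Player overlap with AttackAvoid boosts speed and stores a flee vector; overlap end starts a timer easing speed back down.
; Obstacle hits only set avoidance state and a random vector.
; The looping Flocking timer calls an empty event, and all steering, including line-trace avoidance and fleeing, is disconnected, so the fish never turns.
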(event OnComponentHit(ObstacleAvoiding)
  (params (HitComponent :type Primitive%20Component%20Object%20Reference) (OtherActor :type Actor%20Object%20Reference) (OtherComp :type Primitive%20Component%20Object%20Reference) (NormalImpulse :type Vector :default "0, 0, 0") (Hit :type Hit%20Result%20Structure%20%28by%20ref%29))
  (Variables|Default|SetHitResult Hit)
  (Variables|States|SetIsAvoidingObstacle true)
  (Variables|States|SetIsSwimmingFree false)
  (if (not (== OtherActor (Game|Player|GetPlayerPawn 0)))
    (Variables|Default|SetRandVec (* (Math|Random|RandomUnitVector) 3.0))))

(event OnComponentBeginOverlap(AttackAvoid)
  (params (OverlappedComponent :type Primitive%20Component%20Object%20Reference) (OtherActor :type Actor%20Object%20Reference) (OtherComp :type Primitive%20Component%20Object%20Reference) (OtherBodyIndex :type Integer) (bFromSweep :type Boolean) (SweepResult :type Hit%20Result%20Structure%20%28by%20ref%29))
  (Variables|States|SetIsChased true)
  (if (== OtherActor (Game|Player|GetPlayerPawn 0))
    (Variables|Default|SetChaseVec (- (Transformation|GetActorLocation) (Transformation|GetActorLocation OtherActor)))
    (Variables|Default|SetSpeed 5e+02)
    (if (Utilities|Time|IsTimerActivebyHandle (Variables|Default|GetFishSpeedDecreaseHandle))
      (Utilities|Time|ClearandInvalidateTimerbyHandle (Variables|Default|GetFishSpeedDecreaseHandle)))))

(event OnComponentEndOverlap(AttackAvoid)
  (params (OverlappedComponent :type Primitive%20Component%20Object%20Reference) (OtherActor :type Actor%20Object%20Reference) (OtherComp :type Primitive%20Component%20Object%20Reference) (OtherBodyIndex :type Integer))
  (if (Utilities|Time|IsTimerActivebyHandle (Variables|Default|GetFishSpeedDecreaseHandle))
    (Utilities|Time|ClearandInvalidateTimerbyHandle (Variables|Default|GetFishSpeedDecreaseHandle)))
  (bind _returnvalue (Utilities|Time|SetTimerbyFunctionName 0 "SlowDown" (Variables|Default|GetTimeTick) true))
  (Variables|Default|SetFishSpeedDecreaseHandle _returnvalue))

(event Custom|Flocking)

(event Custom|SlowDown
  (bind _output_get (Variables|Default|SetSpeed (Math|Interpolation|FInterptoConstant (Variables|Default|GetSpeed) 2e+02 (Variables|Default|GetTimeTick) 1e+02)))
  (if (== _output_get 2e+02)
    (Variables|States|SetIsChased false)
    (Utilities|Time|ClearandInvalidateTimerbyHandle (Variables|Default|GetFishSpeedDecreaseHandle))))

(event EventBeginPlay
  (Utilities|Time|SetTimerbyFunctionName self "Flocking" (Variables|Default|GetTimeTick) true))

(event EventTick
  (params (DeltaSeconds :type Float%20%28single-precision%29))
  (bind _returnvalue (Transformation|GetActorLocation))
  (Transformation|SetWorldLocation (Variables|Default|GetFish) (Math|Vector|Lerp(Vector) _returnvalue (+ _returnvalue (* (Transformation|GetActorForwardVector) (Variables|Default|GetSpeed))) (Variables|Default|GetTimeTick)) true false))

(fn ConstructionScript)