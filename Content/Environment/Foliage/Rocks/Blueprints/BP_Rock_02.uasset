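; BP_Rock_02 is a breakable rock that drops items when its durability runs out.
; Its TakeDamage event subtracts the incoming amount from Durability and, at zero or below, passes ItemsToSpawn to SpawnItems.
; SpawnItems spawns each listed class slightly above the rock, enables physics on its ItemMesh, then destroys the rock.
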(event EventBeginPlay)

(event Collision|EventActorBeginOverlap
  (params (OtherActor :type Actor%20Object%20Reference)))

(event EventTick
  (params (DeltaSeconds :type Float%20%28single-precision%29)))

(event EventTakeDamage
  (params (Amount :type Float%20%28single-precision%29))
  (bind _output_get (Variables|Default|SetDurability (- (Variables|Default|GetDurability) Amount)))
  (if (<= _output_get 0.0)
    (CallFunction|SpawnItems (Variables|Default|GetItemsToSpawn))))

(event EventSpawnItems
  (params (Items%20Array :type Array%20of%20Base%20Item%20BP%20Class%20References))
  (for _array_element Items%20Array
    (bind _returnvalue (Game|SpawnActorfromClass _array_element (Math|Transform|MakeTransform (+ (Transformation|GetActorLocation) "0, 0,15.000000") "0, 0, 0" "1,1,1") "Undefined" 0 0))
    (Physics|SetSimulatePhysics (Variables|/Game/Inventory/Items/Blueprints/Items/BaseItem_BP.BaseItem_BP_C|GetItemMesh _returnvalue) true))
  (Actor|DestroyActor))

(fn ConstructionScript)