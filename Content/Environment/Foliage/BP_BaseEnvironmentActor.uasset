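; Base harvestable environment actor that takes damage from a matching tool type and drops items when its health is depleted.
; On BeginPlay it resolves DropoutItemsIndexes into item rows from ItemsDataTable and stores MaxHealth.
; MakeDamage plays a hit sound for any tool, but the wrong one deals no damage and triggers a throttled player hint.
; At zero health it spawns each BaseItem_BP drop above itself, calls TraceDown, then destroys itself.
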(event EventBeginPlay
  (CallFunction|FillDropoutItems)
  (Variables|Default|SetMaxHealth (Variables|Default|GetHealth)))

(event Collision|EventActorBeginOverlap
  (params (OtherActor :type Actor%20Object%20Reference)))

(event EventTick
  (params (DeltaSeconds :type Float%20%28single-precision%29)))

(event EventMakeDamage
  (params (DamageValue :type Float%20%28single-precision%29) (DamagerType :type ToolType%20Enum :default "NewEnumerator2") (ActiveItem :type Base%20in%20Hand%20Item%20BP%20Object%20Reference))
  (bind _damagertooltype (Variables|Default|GetDamagerToolType))
  (if (Utilities|Enum|Equal(Enum) DamagerType _damagertooltype)
    (CallFunction|DecreaseHealth DamageValue)
    (else
      (Utilities|FlowControl|Sequence
        (:then_0
          _)
        (:then_1
          (Utilities|FlowControl|DoOnce false :!label _label
            (:Completed
              (Class|PlayerStatistics|ShowSentence(Message) (Game|GetPlayerCharacter 0) "Your voice:" "It's wrong tool. I should use other" 3.0 true)
              (Utilities|FlowControl|Delay 7.0)
              (goto _label Reset)))))))
  (Default|PlayHitSound ActiveItem _damagertooltype))

(fn ConstructionScript)

(fn DecreaseHealth
  (params (B :type Float%20%28single-precision%29))
  (if (> (- (Variables|Default|GetHealth) B) 0.0)
    (bind _output_get (Variables|Default|SetHealth (- (Variables|Default|GetHealth) B)))
    (Development|PrintString (Utilities|String|ToString(Float) _output_get))
    (else
      (CallFunction|SpawnDropoutItems)
      (Actor|DestroyActor))))

(fn FillDropoutItems
  (for _array_element (Variables|Default|GetDropoutItemsIndexes)
    (bind _outrownames (DataTable|GetDataTableRowNames "/Game/Inventory/Items/Blueprints/ItemsDataTable.ItemsDataTable"))
    (bind _array_element_2 (Utilities|Array|ForEachLoopwithBreak _outrownames :!label _label)
      (:LoopBody
        (bind _returnvalue (Utilities|GetDataTableRow "/Game/Inventory/Items/Blueprints/ItemsDataTable.ItemsDataTable" _array_element_2)
          (:then
            (if (== (.ID (Utilities|Struct|BreakItem _returnvalue)) _array_element)
              (Utilities|Array|Add (Variables|Default|GetDropoutItems) _returnvalue)
              (Development|PrintString (.Name (Utilities|Struct|BreakItem _returnvalue)))
              (goto _label Break))))))))

(fn SpawnDropoutItems
  (bind _returnvalue (Transformation|GetActorTransform))
  (bind (_location _rotation) (Math|Transform|BreakTransform _returnvalue))
  (bind (_x _y _z) (Math|Vector|BreakVector _location))
  (for _array_element (Variables|Default|GetDropoutItems)
    (bind _returnvalue_2 (Game|SpawnActorfromClass (.Class (Utilities|Struct|BreakItem _array_element)) (Math|Transform|MakeTransform (Math|Vector|MakeVector _x _y (+ _z 1e+02)) _rotation) "Undefined" 0 0))
    (bind _asbase_item_bp (Utilities|Casting|CastToBaseItem_BP _returnvalue_2))
    (Default|SetItemProps _asbase_item_bp _array_element)
    (Default|TraceDown _asbase_item_bp)))