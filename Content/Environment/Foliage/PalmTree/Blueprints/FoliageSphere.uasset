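; Proximity sphere actor that follows its owner and swaps instanced foliage for BP_PalmTree_05 actors around it.
; Each tick it sweeps to the owner's location, so sphere hits on instanced meshes spawn a palm Blueprint at that instance's transform and remove the instance.
; Swaps are tracked in ActiveFoliages; beyond a fixed distance, the actor is destroyed and the instance re-added to the foliage actor's first instanced component.
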(event OnComponentHit(Sphere)
  (params (HitComponent :type Primitive%20Component%20Object%20Reference) (OtherActor :type Actor%20Object%20Reference) (OtherComp :type Primitive%20Component%20Object%20Reference) (NormalImpulse :type Vector :default "0, 0, 0") (Hit :type Hit%20Result%20Structure%20%28by%20ref%29))
  (bind (_bblockinghit _binitialoverlap _time _distance _location _impactpoint _normal _impactnormal _physmat _hitactor _hitcomponent _hitbonename _hititem) (Collision|BreakHitResult Hit))
  (Development|PrintString "Sphere Hit" true true "(R=0.000000,G=0.660000,B=1.000000,A=1.000000)" 5.0)
  (bind _asinstanced_static_mesh_component (Utilities|Casting|CastToInstancedStaticMeshComponent _hitcomponent))
  (bind _returnvalue (Game|SpawnActorfromClass "/Game/Environment/Foliage/PalmTree/Blueprints/BP_PalmTree_05.BP_PalmTree_05_C" (.OutInstanceTransform (Components|InstancedStaticMesh|GetInstanceTransform _asinstanced_static_mesh_component _hititem false)) "AlwaysSpawn" 0 0))
  (Utilities|Array|Add (Variables|Default|GetActiveFoliages) (Utilities|Struct|MakeFoliageStruct _returnvalue _hitactor 0 (.OutInstanceTransform (Components|InstancedStaticMesh|GetInstanceTransform _asinstanced_static_mesh_component _hititem false))))
  (Class|InstancedStaticMeshComponent|RemoveInstance _asinstanced_static_mesh_component _hititem))

(event EventBeginPlay)

(event Collision|EventActorBeginOverlap
  (params (OtherActor :type Actor%20Object%20Reference)))

(event EventTick
  (params (DeltaSeconds :type Float%20%28single-precision%29))
  (bind _myowner (Variables|Default|GetMyOwner))
  (Utilities|IsValid _myowner
    (:Is%20Valid
      (Transformation|SetActorLocation (Transformation|GetActorLocation _myowner) true false)
      (Development|PrintString (Utilities|String|ToString(Integer) (Utilities|Array|Length (Variables|Default|GetActiveFoliages))) true true "(R=0.000000,G=0.660000,B=1.000000,A=1.000000)" 0.0)
      (for _array_element (Variables|Default|GetActiveFoliages)
        (if (> (Math|Vector|VectorLength (- (.Location (Math|Transform|BreakTransform (.Transform (Utilities|Struct|BreakFoliageStruct _array_element)))) (- (Transformation|GetActorLocation) "0.000000, 0,45.000000"))) 4e+02)
          (Actor|DestroyActor (.FoliageBP (Utilities|Struct|BreakFoliageStruct _array_element)))
          (Components|InstancedStaticMesh|AddInstance (Utilities|Array|Get(acopy) (Actor|GetComponentsByClass (.FoliageActor (Utilities|Struct|BreakFoliageStruct _array_element)) "/Script/Foliage.FoliageInstancedStaticMeshComponent") (.StaticMeshIndex (Utilities|Struct|BreakFoliageStruct _array_element))) (.Transform (Utilities|Struct|BreakFoliageStruct _array_element)))
          (Utilities|Array|RemoveItem (Variables|Default|GetActiveFoliages) _array_element))))))

(fn ConstructionScript)