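; AI controller for child characters that runs Child_BT and periodically triggers a chase among the children.
; Tick counts a timer down from StartTimerValue and resets it when it drops below zero.
; On each reset it loops over all Child1AI_BP actors, re-rolling a random index per iteration.
; The first match calls StartChasingRandomChild with the full list, so some cycles may start no chase.
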(event EventBeginPlay
  (AI|RunBehaviorTree "/Game/AI/Human/Child/Child_BT.Child_BT")
  (Variables|Default|SetTimer (Variables|Default|GetStartTimerValue)))

(event EventTick
  (params (DeltaSeconds :type Float%20%28single-precision%29))
  (bind _output_get (Variables|Default|SetTimer (- (Variables|Default|GetTimer) DeltaSeconds)))
  (if (< _output_get 0.0)
    (Variables|Default|SetTimer (Variables|Default|GetStartTimerValue))
    (bind _outactors (Actor|GetAllActorsOfClass "/Game/AI/Human/Child/Child1AI_BP.Child1AI_BP_C"))
    (bind (_array_element _array_index) (Utilities|Array|ForEachLoopwithBreak _outactors :!label _label)
      (:LoopBody
        (if (== _array_index (Math|Random|RandomIntegerinRange 0 (- (Utilities|Array|Length _outactors) 1)))
          (Default|StartChasingRandomChild _array_element _outactors)
          (goto _label Break))))))

(fn ConstructionScript)