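; AI controller for the bear animal that runs the BearAI_BT behavior tree on BeginPlay and initializes a countdown timer.
; A disconnected graph section would count the timer down, reset it, and try to make a random Child1AI_BP actor start chasing another child.
; That section never runs, and Tick is empty, so the behavior tree is the only active logic.
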(event EventBeginPlay
  (AI|RunBehaviorTree "/Game/AI/Animal/Bear/BearAI_BT.BearAI_BT")
  (Variables|Default|SetTimer (Variables|Default|GetStartTimerValue)))

(event EventTick
  (params (DeltaSeconds :type Float%20%28single-precision%29)))

(fn ConstructionScript)