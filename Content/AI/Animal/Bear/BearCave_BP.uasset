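; Bear cave actor that serves as the sleeping area for one referenced bear.
; On BeginPlay it registers itself as that bear's Cave.
; When the bear begins overlapping the Box component, it flags the bear as in the cave and gives it a random sleep point within the box extent around the actor's location.
; Nothing here clears the flag when the bear leaves.
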(event OnComponentBeginOverlap(Box)
  (params (OverlappedComponent :type Primitive%20Component%20Object%20Reference) (OtherActor :type Actor%20Object%20Reference) (OtherComp :type Primitive%20Component%20Object%20Reference) (OtherBodyIndex :type Integer) (bFromSweep :type Boolean) (SweepResult :type Hit%20Result%20Structure%20%28by%20ref%29))
  (bind _bear (Variables|Default|GetBear))
  (if (== OtherActor _bear)
    (Variables|/Game/AI/Animal/Bear/AIBear_BP.AIBear_BP_C|SetIsInCave _bear true)
    (Variables|/Game/AI/Animal/Bear/AIBear_BP.AIBear_BP_C|SetPointToSleep (Variables|Default|GetBear) (Math|Random|RandomPointinBoundingBox (Transformation|GetActorLocation) (Components|Box|GetScaledBoxExtent (Variables|Default|GetBox))))))

(event EventBeginPlay
  (Variables|/Game/AI/Animal/Bear/AIBear_BP.AIBear_BP_C|SetCave (Variables|Default|GetBear) self))

(event Collision|EventActorBeginOverlap
  (params (OtherActor :type Actor%20Object%20Reference)))

(event EventTick
  (params (DeltaSeconds :type Float%20%28single-precision%29)))

(fn ConstructionScript)