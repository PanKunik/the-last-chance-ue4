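; Bear AI animal Blueprint that builds on a parent class and adds a raw meat item and wake-up handling.
; On BeginPlay it runs the parent logic, then fills its Item from the RawMeat row of the items data table.
; WakeUp clears the sleeping flag immediately, then switches the AI state after a configurable delay.
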(event Custom|WakeUp
  (Variables|Default|SetIsSleeping false)
  (Utilities|FlowControl|Delay (Variables|Default|GetWakeupDelay))
  (Variables|Default|SetState "NewEnumerator2"))

(event EventBeginPlay
  (|CallParentFunction)
  (bind _returnvalue (Utilities|GetDataTableRow "/Game/Inventory/Items/Blueprints/ItemsDataTable.ItemsDataTable" "RawMeat")
    (:then
      (Variables|Default|SetItem (Utilities|Struct|MakeItem (.ID (Utilities|Struct|BreakItem _returnvalue)) (.Name (Utilities|Struct|BreakItem _returnvalue)) (.Stackable (Utilities|Struct|BreakItem _returnvalue)) (.Type (Utilities|Struct|BreakItem _returnvalue)) 3 (.MaxCount (Utilities|Struct|BreakItem _returnvalue)) (.Icon (Utilities|Struct|BreakItem _returnvalue)) (.Class (Utilities|Struct|BreakItem _returnvalue)) (.IsPickupable (Utilities|Struct|BreakItem _returnvalue)))))))

(event Collision|EventActorBeginOverlap
  (params (OtherActor :type Actor%20Object%20Reference))
  (|CallParentFunction OtherActor) ; This node is disabled and will not be called.\nDrag off pins to build functionality.
)

(event EventTick
  (params (DeltaSeconds :type Float%20%28single-precision%29))
  (|CallParentFunction DeltaSeconds) ; This node is disabled and will not be called.\nDrag off pins to build functionality.
)

(fn ConstructionScript
  (|CallParentFunction))