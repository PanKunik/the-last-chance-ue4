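; Campfire item that burns wood and cooks items, with a billboard HUD showing logs and burn time.
; Ignite starts a looping Fire timer that drains BurnTime, scales the flame and drives roasting and boiling/burning timers, pausing them when fuel runs out.
; An attached grille enables roasting, which swaps the item for its roasted class.
; PutItem sockets clay bars for burning or cauldrons for boiling; AttackLogs manages refuelling through a DoOnce.
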(event Custom|Fire
  ;[1 1 1] FireUp Event
  (if (> (Variables|Burning|GetBurnTime) 0.0)
    (Utilities|FlowControl|Sequence
      (:then_0
        (if (> (Variables|Burning|GetBurnTime) (Variables|Burning|GetExpirationTime))
          (Transformation|SetWorldScale3D (Variables|Default|GetFire_PS) (Math|Vector|MakeVector (Math|Interpolation|FInterptoConstant (Variables|Burning|GetScale) 3.0 (Variables|Burning|GetTimeTick) 0.25) (Math|Interpolation|FInterptoConstant (Variables|Burning|GetScale) 3.0 (Variables|Burning|GetTimeTick) 0.25) (Math|Interpolation|FInterptoConstant (Variables|Burning|GetScale) 3.0 (Variables|Burning|GetTimeTick) 0.25)))
          (Variables|Burning|SetScale (Math|Interpolation|FInterptoConstant (Variables|Burning|GetScale) 3.0 (Variables|Burning|GetTimeTick) 0.25))
          (Variables|Burning|SetBurnTime (Math|Interpolation|FInterptoConstant (Variables|Burning|GetBurnTime) 0.0 (Variables|Burning|GetTimeTick) 1.0))
          (else
            (Transformation|SetWorldScale3D (Variables|Default|GetFire_PS) (Math|Vector|MakeVector (Math|Interpolation|FInterptoConstant (Variables|Burning|GetScale) 0.0 (Variables|Burning|GetTimeTick) 0.25) (Math|Interpolation|FInterptoConstant (Variables|Burning|GetScale) 0.0 (Variables|Burning|GetTimeTick) 0.25) (Math|Interpolation|FInterptoConstant (Variables|Burning|GetScale) 0.0 (Variables|Burning|GetTimeTick) 0.25)))
            (Variables|Burning|SetScale (Math|Interpolation|FInterptoConstant (Variables|Burning|GetScale) 0.0 (Variables|Burning|GetTimeTick) 0.25))
            (Variables|Burning|SetBurnTime (Math|Interpolation|FInterptoConstant (Variables|Burning|GetBurnTime) 0.0 (Variables|Burning|GetTimeTick) 1.0)))))
      (:then_1
        (if (Variables|Default|GetCanItemBeRoasted)
          (if (Utilities|Time|IsTimerActivebyHandle (Variables|Default|GetRoasting_TH))
            (Utilities|Time|UnpauseTimerbyHandle (Variables|Default|GetRoasting_TH))
            (else
              (bind _returnvalue (Utilities|Time|SetTimerbyFunctionName self "Roasting" (Variables|Burning|GetTimeTick) true))
              (Variables|Default|SetRoasting_TH _returnvalue)))))
      (:then_2
        (if (or (Variables|Default|GetCanItemBeBurned) (Variables|Default|GetCanItemBeBoiled))
          (if (Utilities|Time|IsTimerActivebyHandle (Variables|Default|GetBoilingOrBurning_TH))
            (Utilities|Time|UnpauseTimerbyHandle (Variables|Default|GetBoilingOrBurning_TH))
            (else
              (bind _returnvalue_2 (Utilities|Time|SetTimerbyFunctionName self "BoilingOrBurning" (Variables|Burning|GetTimeTick) true))
              (Variables|Default|SetBoilingOrBurning_TH _returnvalue_2))))))
    (else
      (Utilities|Time|ClearandInvalidateTimerbyHandle (Variables|Burning|GetBurning_TH))
      (Components|Activation|SetActive (Variables|Default|GetFire_PS) false false)
      (Variables|Burning|SetScale 0.0)
      (Rendering|SetVisibility (Variables|Default|GetItemMesh) false false)
      (Variables|Fuel|SetWoodItem 0)
      (Transformation|AddLocalOffset (Variables|Default|GetFire_PS) "0, 0,-20.000000" false false)
      (Utilities|FlowControl|Sequence
        (:then_0
          (Utilities|FlowControl|DoOnce true) ; enters at Reset
        )
        (:then_1
          (if (Utilities|Time|IsTimerActivebyHandle (Variables|Default|GetRoasting_TH))
            (Utilities|Time|PauseTimerbyHandle (Variables|Default|GetRoasting_TH))))
        (:then_2
          (if (Utilities|Time|IsTimerActivebyHandle (Variables|Default|GetBoilingOrBurning_TH))
            ;[1 1 1] Event RoastItem
            (Utilities|Time|PauseTimerbyHandle (Variables|Default|GetBoilingOrBurning_TH))))))))

(event Custom|RotateHUD
  (bind _returnvalue (Game|GetPlayerCharacter 0))
  (bind _campfire_hud (Variables|Default|GetCampfire_HUD))
  ;[1 1 1] Rotating HUD to players rotation (Timer)
  (Utilities|IsValid _returnvalue
    (:Is%20Valid
      (Transformation|SetWorldRotation _campfire_hud (Math|Rotator|FindLookatRotation (Transformation|GetWorldLocation (Variables|Default|GetCampfire_HUD)) (Transformation|GetWorldLocation (Variables|/Script/Engine.Character|GetCapsuleComponent _returnvalue))) false false)
      (bind _asumg_bw_items_hud (Utilities|Casting|CastToUMG_BW_ItemsHUD (UserInterface|GetUserWidgetObject _campfire_hud)))
      (Variables|/Game/Inventory/HUD/ItemsHUD/UMG_BW_ItemsHUD.UMG_BW_ItemsHUD_C|SetHUD_Text _asumg_bw_items_hud (Utilities|Text|ToText(String) (Utilities|String|Append "Wood logs:" (Utilities|String|ToString(Integer) (Variables|Fuel|GetWoodItem)) "/1" "Burn time: " (Utilities|String|ToString(Integer) (Math|Float|Round (Variables|Burning|GetBurnTime))) " s"))))))

(event Custom|Roasting
  ;[1 1 1] Event RoastItem
  (bind _output_get (Variables|Burning|SetRoastTime (Math|Interpolation|FInterptoConstant (Variables|Burning|GetRoastTime) 0.0 (Variables|Burning|GetTimeTick) 1.0)))
  (if (> _output_get 0.0)
    (Development|PrintString "Update roast bar")
    (else
      (Utilities|FlowControl|DoOnce false
        (:Completed
          (bind _asbase_item_bp (Utilities|Casting|CastToBaseItem_BP (Variables|Default|GetRoastingItem)))
          (bind _roasteditem (Default|ChangeRoastedItem _asbase_item_bp))
          (bind _returnvalue (Game|SpawnActorfromClass _roasteditem (Transformation|GetActorTransform (Variables|Default|GetRoastingItem)) "Undefined" 0 0))
          (Actor|DestroyActor (Variables|Default|GetRoastingItem))
          (Variables|Default|SetRoastingItem _returnvalue)
          (Utilities|Time|ClearandInvalidateTimerbyHandle (Variables|Default|GetRoasting_TH))
          (Variables|Default|SetCanItemBeRoasted false))))))

(event Custom|BoilingOrBurning
  (if (Variables|Default|GetCanItemBeBurned)
    (bind _output_get (Variables|Burning|SetBurningOrBoilingTime (Math|Interpolation|FInterptoConstant (Variables|Burning|GetBurningOrBoilingTime) 0.0 (Variables|Burning|GetTimeTick) 1.0)))
    (if (not (> _output_get 0.0))
      (CallFunction|Burned)
      (Utilities|Time|ClearandInvalidateTimerbyHandle (Variables|Default|GetBoilingOrBurning_TH) :!label _label))
    (elif (Variables|Default|GetCanItemBeBoiled)
      (bind _output_get_2 (Variables|Burning|SetBurningOrBoilingTime (Math|Interpolation|FInterptoConstant (Variables|Burning|GetBurningOrBoilingTime) 0.0 (Variables|Burning|GetTimeTick) 1.0)))
      (if (not (> _output_get_2 0.0))
        (CallFunction|Boiled)
        (goto _label)))))

(event Custom|ResetBoilingOrBurningDoOnce
  (Utilities|FlowControl|DoOnce false) ; enters at Reset
)

(event Custom|Boiled
  (Variables|Default|SetCanItemBeBoiled false)
  (bind _ascauldron_bp (Utilities|Casting|CastToCauldron_BP (Variables|Default|GetBoilingBurningItem)))
  (Default|Ready _ascauldron_bp))

(event Custom|Burned
  (bind _boilingburningitem (Variables|Default|GetBoilingBurningItem))
  (Variables|Default|SetCanItemBeBurned false)
  (Class|UsingItemsInterface|ChangeBurnedItem(Message) _boilingburningitem)
  (bind _asbase_item_bp (Utilities|Casting|CastToBaseItem_BP _boilingburningitem))
  (Default|SetItemProps _asbase_item_bp (Utilities|Struct|MakeItem (.ID (Utilities|Struct|BreakItem (Variables|/Game/Inventory/Items/Blueprints/Items/BaseItem_BP.BaseItem_BP_C|GetItemProps _asbase_item_bp))) (.Name (Utilities|Struct|BreakItem (Variables|/Game/Inventory/Items/Blueprints/Items/BaseItem_BP.BaseItem_BP_C|GetItemProps _asbase_item_bp))) (.Stackable (Utilities|Struct|BreakItem (Variables|/Game/Inventory/Items/Blueprints/Items/BaseItem_BP.BaseItem_BP_C|GetItemProps _asbase_item_bp))) (.Type (Utilities|Struct|BreakItem (Variables|/Game/Inventory/Items/Blueprints/Items/BaseItem_BP.BaseItem_BP_C|GetItemProps _asbase_item_bp))) (.Count (Utilities|Struct|BreakItem (Variables|/Game/Inventory/Items/Blueprints/Items/BaseItem_BP.BaseItem_BP_C|GetItemProps _asbase_item_bp))) (.MaxCount (Utilities|Struct|BreakItem (Variables|/Game/Inventory/Items/Blueprints/Items/BaseItem_BP.BaseItem_BP_C|GetItemProps _asbase_item_bp))) (.Icon (Utilities|Struct|BreakItem (Variables|/Game/Inventory/Items/Blueprints/Items/BaseItem_BP.BaseItem_BP_C|GetItemProps _asbase_item_bp))) (.Class (Utilities|Struct|BreakItem (Variables|/Game/Inventory/Items/Blueprints/Items/BaseItem_BP.BaseItem_BP_C|GetItemProps _asbase_item_bp))) true)))

(event EventBeginPlay
  ;[1 1 1] Event BeginPlay -> Attach Coal (Fuel) to campfire
  (|CallParentFunction)
  (Variables|Fuel|SetWoodItem 1)
  (Variables|Default|SetCanItemBeRoasted false)
  (bind _returnvalue (Game|SpawnActorfromClass "/Game/Inventory/Items/Blueprints/Items/Resources/CampfireCoal_BP.CampfireCoal_BP_C" (Math|Transform|MakeTransform "0, 0, 0") "Undefined" 0 0))
  (bind _output_get (Variables|Fuel|SetFuel _returnvalue))
  (Transformation|AttachActorToActor _output_get self "CampfireGrille" "KeepRelative" "KeepRelative" "KeepRelative" true)
  (Utilities|Time|SetTimerbyFunctionName self "RotateHUD" (Variables|Burning|GetTimeTick) true))

(event Collision|EventActorBeginOverlap
  (params (OtherActor :type Actor%20Object%20Reference))
  (|CallParentFunction OtherActor) ; This node is disabled and will not be called.\nDrag off pins to build functionality.
)

(event EventIgnite
  ;[1 1 1] Event Ignite
  (Variables|Burning|SetTimeTick 0.05)
  (if (> (Variables|Burning|GetBurnTime) 0.0)
    (if (not (Utilities|Time|IsTimerActivebyHandle (Variables|Burning|GetBurning_TH)))
      (bind _returnvalue (Utilities|Time|SetTimerbyFunctionName self "Fire" (Variables|Burning|GetTimeTick) true))
      (Variables|Burning|SetBurning_TH _returnvalue)
      (Components|Activation|SetActive (Variables|Default|GetFire_PS) true true))))

(event EventAttachGrille
  ;[1 1 1] Event AttachGrille
  (Utilities|FlowControl|DoOnce false
    (:Completed
      (bind _returnvalue (Game|SpawnActorfromClass "/Game/Inventory/Items/Blueprints/Items/In_Hand_Items/Utilities/CampfireGrille_BP.CampfireGrille_BP_C" (Math|Transform|MakeTransform "0, 0, 0") "Undefined" 0 0))
      (Transformation|AttachActorToActor _returnvalue self "CampfireGrille" "KeepRelative" "KeepWorld" "KeepRelative" true)
      (bind _output_get (Variables|Default|SetGrilleRotation (Math|Rotator|MakeRotator 0.0 0.0 (+ (.Yaw (Math|Rotator|BreakRotator (Transformation|GetActorRotation (Game|GetPlayerCharacter 0)))) 9e+01))))
      (Transformation|SetActorRotation _returnvalue _output_get)
      (Variables|Default|SetIsGrilleAttached true))))

(event EventAttackLogs
  ;[1 1 1] FireUp Event
  (Utilities|FlowControl|DoOnce true
    (:Completed
      (Rendering|SetVisibility (Variables|Default|GetItemMesh) true false)
      (Variables|Burning|SetBurnTime (+ (Variables|Burning|GetBurnTime) 5e+01))
      (Variables|Fuel|SetWoodItem 1)
      (Transformation|AddLocalOffset (Variables|Default|GetFire_PS) "0, 0,20.000000" false false))))

(event EventRoastItem
  (params (Item :type Actor%20Class%20Reference))
  ;[1 1 1] Event RoastItem
  (if (Variables|Default|GetIsGrilleAttached)
    (if (not (Utilities|IsValid (Variables|Default|GetRoastingItem)))
      (Variables|Default|SetCanItemBeRoasted true)
      (Variables|Burning|SetRoastTime 1.1e+02)
      (bind _returnvalue (Game|SpawnActorfromClass Item (Math|Transform|MakeTransform "0, 0, 0") "Undefined" self 0))
      (bind _output_get (Variables|Default|SetRoastingItem _returnvalue))
      (Transformation|AddActorLocalOffset _output_get (- (Transformation|GetSocketLocation (Variables|Default|GetItemMesh) "MaterialSocket") (Transformation|GetActorLocation)) false false)
      (Transformation|SetActorRotation (Variables|Default|GetRoastingItem) (Variables|Default|GetGrilleRotation))
      (Transformation|AttachActorToActor (Variables|Default|GetRoastingItem) self "MaterialSocket" "KeepRelative" "KeepWorld" "KeepRelative" true)
      (bind _asbase_item_bp (Utilities|Casting|CastToBaseItem_BP (Variables|Default|GetRoastingItem)))
      (Default|SetItemProps _asbase_item_bp (Utilities|Struct|MakeItem (.ID (Utilities|Struct|BreakItem (Variables|/Game/Inventory/Items/Blueprints/Items/BaseItem_BP.BaseItem_BP_C|GetItemProps _asbase_item_bp))) (.Name (Utilities|Struct|BreakItem (Variables|/Game/Inventory/Items/Blueprints/Items/BaseItem_BP.BaseItem_BP_C|GetItemProps _asbase_item_bp))) (.Stackable (Utilities|Struct|BreakItem (Variables|/Game/Inventory/Items/Blueprints/Items/BaseItem_BP.BaseItem_BP_C|GetItemProps _asbase_item_bp))) (.Type (Utilities|Struct|BreakItem (Variables|/Game/Inventory/Items/Blueprints/Items/BaseItem_BP.BaseItem_BP_C|GetItemProps _asbase_item_bp))) (.Count (Utilities|Struct|BreakItem (Variables|/Game/Inventory/Items/Blueprints/Items/BaseItem_BP.BaseItem_BP_C|GetItemProps _asbase_item_bp))) (.MaxCount (Utilities|Struct|BreakItem (Variables|/Game/Inventory/Items/Blueprints/Items/BaseItem_BP.BaseItem_BP_C|GetItemProps _asbase_item_bp))) (.Icon (Utilities|Struct|BreakItem (Variables|/Game/Inventory/Items/Blueprints/Items/BaseItem_BP.BaseItem_BP_C|GetItemProps _asbase_item_bp))) "/Game/Inventory/Items/Blueprints/Items/In_Hand_Items/Food/F_Meat_BP.F_Meat_BP_C" false))
      (Utilities|FlowControl|DoOnce false) ; enters at Reset
    )))

(event EventPutItem
  (params (Class :type Actor%20Class%20Reference))
  (if (not (Utilities|IsValid (Variables|Default|GetBoilingBurningItem)))
    (Utilities|FlowControl|DoOnce false
      (:Completed
        (if (== Class "/Game/Inventory/Items/Blueprints/Items/Resources/ClayBar_BP.ClayBar_BP_C")
          (Variables|Default|SetCanItemBeBurned true)
          (Variables|Burning|SetBurningOrBoilingTime 3e+01)
          (bind _returnvalue (Game|SpawnActorfromClass Class (Math|Transform|MakeTransform "0, 0, 0") "Undefined" self 0))
          (Variables|Default|SetBoilingBurningItem _returnvalue)
          (Transformation|AddActorLocalOffset (Variables|Default|GetBoilingBurningItem) (- (Transformation|GetSocketLocation (Variables|Default|GetItemMesh) "BurningSocket") (Transformation|GetActorLocation)) false false :!label _label)
          (Transformation|AttachActorToActor (Variables|Default|GetBoilingBurningItem) self "BurningSocket" "KeepRelative" "KeepRelative" "KeepRelative" true)
          (bind _asbase_item_bp (Utilities|Casting|CastToBaseItem_BP (Variables|Default|GetBoilingBurningItem)))
          (Default|SetItemProps _asbase_item_bp (Utilities|Struct|MakeItem (.ID (Utilities|Struct|BreakItem (Variables|/Game/Inventory/Items/Blueprints/Items/BaseItem_BP.BaseItem_BP_C|GetItemProps _asbase_item_bp))) (.Name (Utilities|Struct|BreakItem (Variables|/Game/Inventory/Items/Blueprints/Items/BaseItem_BP.BaseItem_BP_C|GetItemProps _asbase_item_bp))) (.Stackable (Utilities|Struct|BreakItem (Variables|/Game/Inventory/Items/Blueprints/Items/BaseItem_BP.BaseItem_BP_C|GetItemProps _asbase_item_bp))) (.Type (Utilities|Struct|BreakItem (Variables|/Game/Inventory/Items/Blueprints/Items/BaseItem_BP.BaseItem_BP_C|GetItemProps _asbase_item_bp))) (.Count (Utilities|Struct|BreakItem (Variables|/Game/Inventory/Items/Blueprints/Items/BaseItem_BP.BaseItem_BP_C|GetItemProps _asbase_item_bp))) (.MaxCount (Utilities|Struct|BreakItem (Variables|/Game/Inventory/Items/Blueprints/Items/BaseItem_BP.BaseItem_BP_C|GetItemProps _asbase_item_bp))) (.Icon (Utilities|Struct|BreakItem (Variables|/Game/Inventory/Items/Blueprints/Items/BaseItem_BP.BaseItem_BP_C|GetItemProps _asbase_item_bp))) (.Class (Utilities|Struct|BreakItem (Variables|/Game/Inventory/Items/Blueprints/Items/BaseItem_BP.BaseItem_BP_C|GetItemProps _asbase_item_bp))) false))
          (elif (== Class "/Game/Inventory/Items/Blueprints/Items/In_Hand_Items/Utilities/Cauldron_BP.Cauldron_BP_C")
            (Variables|Burning|SetBurningOrBoilingTime 15.0)
            (bind _returnvalue_2 (Game|SpawnActorfromClass Class (Math|Transform|MakeTransform "0, 0, 0") "Undefined" self 0))
            (Variables|Default|SetBoilingBurningItem _returnvalue_2)
            (goto _label)))))))

(fn ConstructionScript
  (|CallParentFunction))