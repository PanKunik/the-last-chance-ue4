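; Campfire inventory item that burns stick and coal fuel and roasts items on an attachable grille.
; Ignite starts a looping Fire timer that drains burn time, scales the flame particles and periodically hides coal meshes on a spawned CampfireCoal_BP actor.
; While burning, a roasting timer counts down, then swaps the item for its roasted class, pausing when the fire dies.
; Another timer turns the widget HUD toward the player and updates fuel readouts.
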(event Custom|Fire
  ;[1 1 1] FireUp Event
  (if (> (Variables|Burning|GetBurnTime) 0.0)
    (Utilities|FlowControl|Sequence
      (:then_0
        (Utilities|FlowControl|DoOnce false
          (:Completed
            (if (> (Variables|Burning|GetBurnTime) 24.0)
              (Variables|Burning|SetExpirationTime 12.0)
              (else
                (Variables|Burning|SetExpirationTime (/ (Variables|Burning|GetBurnTime) 2.0)))))))
      (:then_1
        (if (> (Variables|Burning|GetBurnTime) (Variables|Burning|GetExpirationTime))
          (Transformation|SetWorldScale3D (Variables|Default|GetFire_PS) (Math|Vector|MakeVector (Math|Interpolation|FInterptoConstant (Variables|Burning|GetScale) 3.0 (Variables|Burning|GetTimeTick) 0.25) (Math|Interpolation|FInterptoConstant (Variables|Burning|GetScale) 3.0 (Variables|Burning|GetTimeTick) 0.25) (Math|Interpolation|FInterptoConstant (Variables|Burning|GetScale) 3.0 (Variables|Burning|GetTimeTick) 0.25)))
          (Variables|Burning|SetScale (Math|Interpolation|FInterptoConstant (Variables|Burning|GetScale) 3.0 (Variables|Burning|GetTimeTick) 0.25))
          (Variables|Burning|SetBurnTime (Math|Interpolation|FInterptoConstant (Variables|Burning|GetBurnTime) 0.0 (Variables|Burning|GetTimeTick) 1.0))
          (Variables|Burning|SetElapsed (Math|Interpolation|FInterptoConstant (Variables|Burning|GetElapsed) 6e+01 (Variables|Burning|GetTimeTick) 1.0))
          (else
            (Transformation|SetWorldScale3D (Variables|Default|GetFire_PS) (Math|Vector|MakeVector (Math|Interpolation|FInterptoConstant (Variables|Burning|GetScale) 0.0 (Variables|Burning|GetTimeTick) 0.25) (Math|Interpolation|FInterptoConstant (Variables|Burning|GetScale) 0.0 (Variables|Burning|GetTimeTick) 0.25) (Math|Interpolation|FInterptoConstant (Variables|Burning|GetScale) 0.0 (Variables|Burning|GetTimeTick) 0.25)))
            (Variables|Burning|SetScale (Math|Interpolation|FInterptoConstant (Variables|Burning|GetScale) 0.0 (Variables|Burning|GetTimeTick) 0.25))
            (Variables|Burning|SetBurnTime (Math|Interpolation|FInterptoConstant (Variables|Burning|GetBurnTime) 0.0 (Variables|Burning|GetTimeTick) 1.0))
            (Variables|Burning|SetElapsed (Math|Interpolation|FInterptoConstant (Variables|Burning|GetElapsed) 6e+01 (Variables|Burning|GetTimeTick) 1.0)))))
      (:then_2
        (if (> (Variables|Fuel|GetFuelFill) 0)
          (if (>= (Variables|Burning|GetElapsed) 3e+01)
            (Variables|Burning|SetElapsed (- (Variables|Burning|GetElapsed) 3e+01))
            (CallFunction|HideCoal)
            (Variables|Fuel|SetFuelFill (- (Variables|Fuel|GetFuelFill) 1)))))
      (:then_3
        (if (Variables|Default|GetCanItemBeRoasted)
          (if (Utilities|Time|IsTimerActivebyHandle (Variables|Default|GetRoasting_TH))
            (Utilities|Time|UnpauseTimerbyHandle (Variables|Default|GetRoasting_TH))
            (else
              (bind _returnvalue (Utilities|Time|SetTimerbyFunctionName self "Roasting" (Variables|Burning|GetTimeTick) true))
              (Variables|Default|SetRoasting_TH _returnvalue))))))
    (else
      (Utilities|Time|ClearandInvalidateTimerbyHandle (Variables|Burning|GetBurning_TH))
      (Components|Activation|SetActive (Variables|Default|GetFire_PS) false false)
      (Variables|Burning|SetScale 0.0)
      (Rendering|SetVisibility (Variables|Default|GetSticks) false false)
      (Variables|Fuel|SetSticksItem 0)
      (Variables|Burning|SetElapsed 0.0)
      (Transformation|AddLocalOffset (Variables|Default|GetFire_PS) "0, 0,-20.000000" false false)
      (Utilities|FlowControl|Sequence
        (:then_0
          (CallFunction|ResetFiringDoOnce))
        (:then_1
          (Utilities|FlowControl|DoOnce true) ; enters at Reset
        )
        (:then_2
          (if (Utilities|Time|IsTimerActivebyHandle (Variables|Default|GetRoasting_TH))
            (Utilities|Time|PauseTimerbyHandle (Variables|Default|GetRoasting_TH))))))))

(event Custom|HideCoal
  ;[1 1 1] Event HideCoal -> When they burn
  (bind _ascampfire_coal_bp (Utilities|Casting|CastToCampfireCoal_BP (Variables|Fuel|GetFuel)))
  (switch int (- (Variables|Fuel|GetFuelFill) 1)
    (:0
      (Rendering|SetVisibility (Variables|/Game/Inventory/Items/Blueprints/Items/BaseItem_BP.BaseItem_BP_C|GetItemMesh _ascampfire_coal_bp) false false))
    (:1
      (Rendering|SetVisibility (Variables|/Game/Inventory/Items/Blueprints/Items/Resources/CampfireCoal_BP.CampfireCoal_BP_C|GetStaticMesh _ascampfire_coal_bp) false false))
    (:2
      (Rendering|SetVisibility (Variables|/Game/Inventory/Items/Blueprints/Items/Resources/CampfireCoal_BP.CampfireCoal_BP_C|GetStaticMesh1 _ascampfire_coal_bp) false false))
    (:3
      (Rendering|SetVisibility (Variables|/Game/Inventory/Items/Blueprints/Items/Resources/CampfireCoal_BP.CampfireCoal_BP_C|GetStaticMesh2 _ascampfire_coal_bp) false false))
    (:4
      (Rendering|SetVisibility (Variables|/Game/Inventory/Items/Blueprints/Items/Resources/CampfireCoal_BP.CampfireCoal_BP_C|GetStaticMesh3 _ascampfire_coal_bp) false false))
    (:5
      (Rendering|SetVisibility (Variables|/Game/Inventory/Items/Blueprints/Items/Resources/CampfireCoal_BP.CampfireCoal_BP_C|GetStaticMesh4 _ascampfire_coal_bp) false false))
    (:6
      (Rendering|SetVisibility (Variables|/Game/Inventory/Items/Blueprints/Items/Resources/CampfireCoal_BP.CampfireCoal_BP_C|GetStaticMesh5 _ascampfire_coal_bp) false false))
    (:7
      (Rendering|SetVisibility (Variables|/Game/Inventory/Items/Blueprints/Items/Resources/CampfireCoal_BP.CampfireCoal_BP_C|GetStaticMesh6 _ascampfire_coal_bp) false false))
    (:8
      (Rendering|SetVisibility (Variables|/Game/Inventory/Items/Blueprints/Items/Resources/CampfireCoal_BP.CampfireCoal_BP_C|GetStaticMesh7 _ascampfire_coal_bp) false false))
    (:9
      (Rendering|SetVisibility (Variables|/Game/Inventory/Items/Blueprints/Items/Resources/CampfireCoal_BP.CampfireCoal_BP_C|GetStaticMesh8 _ascampfire_coal_bp) false false))
    (:10
      (Rendering|SetVisibility (Variables|/Game/Inventory/Items/Blueprints/Items/Resources/CampfireCoal_BP.CampfireCoal_BP_C|GetStaticMesh9 _ascampfire_coal_bp) false false))))

(event Custom|RotateHUD
  (bind _returnvalue (Game|GetPlayerCharacter 0))
  (bind _campfire_hud (Variables|Default|GetCampfire_HUD))
  ;[1 1 1] Rotating HUD to players rotation (Timer)
  (Utilities|IsValid _returnvalue
    (:Is%20Valid
      (Transformation|SetWorldRotation _campfire_hud (Math|Rotator|MakeRotator 0.0 0.0 (.Yaw (Math|Rotator|BreakRotator (Math|Rotator|FindLookatRotation (Transformation|GetWorldLocation (Variables|Default|GetCampfire_HUD)) (Transformation|GetWorldLocation (Variables|/Script/Engine.Character|GetCapsuleComponent _returnvalue)))))) false false)
      (bind _asumg_bw_campfire_hud (Utilities|Casting|CastToUMG_BW_CampfireHUD (UserInterface|GetUserWidgetObject _campfire_hud)))
      (Variables|/Game/Inventory/HUD/ItemsHUD/UMG_BW_CampfireHUD.UMG_BW_CampfireHUD_C|SetHUD_FuelSticks _asumg_bw_campfire_hud (Utilities|Text|ToText(String) (Utilities|String|Append (Utilities|String|ToString(Integer) (Variables|Fuel|GetSticksItem)) "/1")))
      (Variables|/Game/Inventory/HUD/ItemsHUD/UMG_BW_CampfireHUD.UMG_BW_CampfireHUD_C|SetHUD_FuelCoal _asumg_bw_campfire_hud (Utilities|Text|ToText(String) (Utilities|String|Append (Utilities|String|ToString(Integer) (Variables|Fuel|GetFuelFill)) "/11")))
      (Variables|/Game/Inventory/HUD/ItemsHUD/UMG_BW_CampfireHUD.UMG_BW_CampfireHUD_C|SetHUD_BurnTime _asumg_bw_campfire_hud (Utilities|Text|ToText(String) (Utilities|String|Append (Utilities|String|ToString(Integer) (Math|Float|Round (Variables|Burning|GetBurnTime))) " s")))
      (Variables|/Game/Inventory/HUD/ItemsHUD/UMG_BW_CampfireHUD.UMG_BW_CampfireHUD_C|SetHUD_Name _asumg_bw_campfire_hud (Utilities|Text|ToText(String) (.Name (Utilities|Struct|BreakItem (Variables|Default|GetItemProps)))))
      (Variables|/Game/Inventory/HUD/ItemsHUD/UMG_BW_CampfireHUD.UMG_BW_CampfireHUD_C|SetHUD_ProgressBarValue _asumg_bw_campfire_hud (/ (Variables|Burning|GetBurnTime) (Variables|Burning|GetMaxBurnTime))))))

(event Custom|Roasting
  ;[1 1 1] Event RoastItem
  (bind _output_get (Variables|Burning|SetRoastTime (Math|Interpolation|FInterptoConstant (Variables|Burning|GetRoastTime) 0.0 (Variables|Burning|GetTimeTick) 1.0)))
  (if (> _output_get 0.0)
    (Development|PrintString "Update roast bar")
    (else
      (Utilities|FlowControl|DoOnce false
        (:Completed
          (bind _asbase_item_bp (Utilities|Casting|CastToBaseItem_BP (Variables|Default|GetRoastingItem)))
          (bind _roasteditem (Default|ChangeRoastedItem _asbase_item_bp))
          (bind _returnvalue (Game|SpawnActorfromClass _roasteditem (Transformation|GetActorTransform (Variables|Default|GetRoastingItem)) "Undefined" 0 0))
          (Actor|DestroyActor (Variables|Default|GetRoastingItem))
          (Variables|Default|SetRoastingItem _returnvalue)
          (Utilities|Time|ClearandInvalidateTimerbyHandle (Variables|Default|GetRoasting_TH))
          (Variables|Default|SetCanItemBeRoasted false))))))

(event Custom|ResetFiringDoOnce
  ;[1 1 1] FireUp Event
  (Utilities|FlowControl|DoOnce false) ; enters at Reset
)

(event EventBeginPlay
  ;[1 1 1] Event BeginPlay -> Attach Coal (Fuel) to campfire
  (|CallParentFunction)
  (Variables|Burning|SetMaxBurnTime 3.8e+02)
  (Variables|Burning|SetBurnTime 5e+01)
  (Variables|Fuel|SetSticksItem 1)
  (Variables|Default|SetCanItemBeRoasted false)
  (bind _returnvalue (Game|SpawnActorfromClass "/Game/Inventory/Items/Blueprints/Items/Resources/CampfireCoal_BP.CampfireCoal_BP_C" (Math|Transform|MakeTransform "0, 0, 0") "Undefined" 0 0))
  (bind _output_get (Variables|Fuel|SetFuel _returnvalue))
  (Transformation|AttachActorToActor _output_get self "CampfireGrille" "KeepRelative" "KeepRelative" "KeepRelative" true)
  (Utilities|Time|SetTimerbyFunctionName self "RotateHUD" 0.01 true))

(event Collision|EventActorBeginOverlap
  (params (OtherActor :type Actor%20Object%20Reference))
  (|CallParentFunction OtherActor) ; This node is disabled and will not be called.\nDrag off pins to build functionality.
)

(event EventAttachSticks
  ;[1 1 1] FireUp Event
  (Utilities|FlowControl|DoOnce true
    (:Completed
      (Rendering|SetVisibility (Variables|Default|GetSticks) true false)
      (Variables|Burning|SetBurnTime (+ (Variables|Burning|GetBurnTime) 5e+01))
      (Variables|Fuel|SetSticksItem 1)
      (Transformation|AddLocalOffset (Variables|Default|GetFire_PS) "0, 0,20.000000" false false))))

(event EventAddFuel
  (params (FuelClass :type Actor%20Class%20Reference))
  (bind _fuelitems (Variables|Fuel|GetFuelItems))
  (bind (_fuelobject _fuelcapacity _burntime) (Utilities|Struct|BreakSTR_FuelItem _fuelitems))
  ;[1 1 1] Event AddFuel -> When adding coals
  (Utilities|FlowControl|Sequence
    (:then_0
      (if (== FuelClass _fuelobject)
        (if (< (+ (Variables|Fuel|GetFuelFill) _fuelcapacity) 12)
          (Variables|Fuel|SetFuelFill (+ (Variables|Fuel|GetFuelFill) _fuelcapacity))
          (Variables|Burning|SetBurnTime (+ (Variables|Burning|GetBurnTime) _burntime))
          (bind _ascampfire_coal_bp (Utilities|Casting|CastToCampfireCoal_BP (Variables|Fuel|GetFuel)))
          (switch int (- (Variables|Fuel|GetFuelFill) 1)
            (:0
              (Rendering|SetVisibility (Variables|/Game/Inventory/Items/Blueprints/Items/BaseItem_BP.BaseItem_BP_C|GetItemMesh _ascampfire_coal_bp) true false))
            (:1
              (Rendering|SetVisibility (Variables|/Game/Inventory/Items/Blueprints/Items/Resources/CampfireCoal_BP.CampfireCoal_BP_C|GetStaticMesh _ascampfire_coal_bp) true false))
            (:2
              (Rendering|SetVisibility (Variables|/Game/Inventory/Items/Blueprints/Items/Resources/CampfireCoal_BP.CampfireCoal_BP_C|GetStaticMesh1 _ascampfire_coal_bp) true false))
            (:3
              (Rendering|SetVisibility (Variables|/Game/Inventory/Items/Blueprints/Items/Resources/CampfireCoal_BP.CampfireCoal_BP_C|GetStaticMesh2 _ascampfire_coal_bp) true false))
            (:4
              (Rendering|SetVisibility (Variables|/Game/Inventory/Items/Blueprints/Items/Resources/CampfireCoal_BP.CampfireCoal_BP_C|GetStaticMesh3 _ascampfire_coal_bp) true false))
            (:5
              (Rendering|SetVisibility (Variables|/Game/Inventory/Items/Blueprints/Items/Resources/CampfireCoal_BP.CampfireCoal_BP_C|GetStaticMesh4 _ascampfire_coal_bp) true false))
            (:6
              (Rendering|SetVisibility (Variables|/Game/Inventory/Items/Blueprints/Items/Resources/CampfireCoal_BP.CampfireCoal_BP_C|GetStaticMesh5 _ascampfire_coal_bp) true false))
            (:7
              (Rendering|SetVisibility (Variables|/Game/Inventory/Items/Blueprints/Items/Resources/CampfireCoal_BP.CampfireCoal_BP_C|GetStaticMesh6 _ascampfire_coal_bp) true false))
            (:8
              (Rendering|SetVisibility (Variables|/Game/Inventory/Items/Blueprints/Items/Resources/CampfireCoal_BP.CampfireCoal_BP_C|GetStaticMesh7 _ascampfire_coal_bp) true false))
            (:9
              (Rendering|SetVisibility (Variables|/Game/Inventory/Items/Blueprints/Items/Resources/CampfireCoal_BP.CampfireCoal_BP_C|GetStaticMesh8 _ascampfire_coal_bp) true false))
            (:10
              (Rendering|SetVisibility (Variables|/Game/Inventory/Items/Blueprints/Items/Resources/CampfireCoal_BP.CampfireCoal_BP_C|GetStaticMesh9 _ascampfire_coal_bp) true false))))))
    (:then_1
      (CallFunction|ResetFiringDoOnce))))

(event EventIgnite
  ;[1 1 1] Event Ignite
  (Variables|Burning|SetTimeTick 0.05)
  (if (> (Variables|Burning|GetBurnTime) 0.0)
    (if (not (Utilities|Time|IsTimerActivebyHandle (Variables|Burning|GetBurning_TH)))
      (bind _returnvalue (Utilities|Time|SetTimerbyFunctionName self "Fire" (Variables|Burning|GetTimeTick) true))
      (Variables|Burning|SetBurning_TH _returnvalue)
      (Components|Activation|SetActive (Variables|Default|GetFire_PS) true true))))

(event EventAttachGrille
  ;[1 1 1] Event AttachGrille
  (Utilities|FlowControl|DoOnce false
    (:Completed
      (bind _returnvalue (Game|SpawnActorfromClass "/Game/Inventory/Items/Blueprints/Items/In_Hand_Items/Utilities/CampfireGrille_BP.CampfireGrille_BP_C" (Math|Transform|MakeTransform "0, 0, 0") "Undefined" 0 0))
      (Transformation|AttachActorToActor _returnvalue self "CampfireGrille" "KeepRelative" "KeepWorld" "KeepRelative" true)
      (bind _output_get (Variables|Default|SetGrilleRotation (Math|Rotator|MakeRotator 0.0 0.0 (+ (.Yaw (Math|Rotator|BreakRotator (Transformation|GetActorRotation (Game|GetPlayerCharacter 0)))) 9e+01))))
      (Transformation|SetActorRotation _returnvalue _output_get)
      (Variables|Default|SetIsGrilleAttached true)
      (Transformation|AddLocalOffset (Variables|Default|GetCampfire_HUD) "0, 0,50.000000" false false))))

(event EventRoastItem
  (params (Item :type Actor%20Class%20Reference))
  ;[1 1 1] Event RoastItem
  (if (Variables|Default|GetIsGrilleAttached)
    (if (not (Utilities|IsValid (Variables|Default|GetRoastingItem)))
      (Variables|Default|SetCanItemBeRoasted true)
      (Variables|Burning|SetRoastTime 1.1e+02)
      (bind _returnvalue (Game|SpawnActorfromClass Item (Math|Transform|MakeTransform "0, 0, 0") "Undefined" self 0))
      (bind _output_get (Variables|Default|SetRoastingItem _returnvalue))
      (Transformation|AddActorLocalOffset _output_get (- (Transformation|GetSocketLocation (Variables|Default|GetItemMesh) "MaterialSocket") (Transformation|GetActorLocation)) false false)
      (Transformation|SetActorRotation (Variables|Default|GetRoastingItem) (Variables|Default|GetGrilleRotation))
      (Transformation|AttachActorToActor (Variables|Default|GetRoastingItem) self "MaterialSocket" "KeepRelative" "KeepWorld" "KeepRelative" true)
      (bind _asbase_item_bp (Utilities|Casting|CastToBaseItem_BP (Variables|Default|GetRoastingItem)))
      (Default|SetItemProps _asbase_item_bp (Utilities|Struct|MakeItem (.ID (Utilities|Struct|BreakItem (Variables|/Game/Inventory/Items/Blueprints/Items/BaseItem_BP.BaseItem_BP_C|GetItemProps _asbase_item_bp))) (.Name (Utilities|Struct|BreakItem (Variables|/Game/Inventory/Items/Blueprints/Items/BaseItem_BP.BaseItem_BP_C|GetItemProps _asbase_item_bp))) (.Stackable (Utilities|Struct|BreakItem (Variables|/Game/Inventory/Items/Blueprints/Items/BaseItem_BP.BaseItem_BP_C|GetItemProps _asbase_item_bp))) (.Type (Utilities|Struct|BreakItem (Variables|/Game/Inventory/Items/Blueprints/Items/BaseItem_BP.BaseItem_BP_C|GetItemProps _asbase_item_bp))) (.Count (Utilities|Struct|BreakItem (Variables|/Game/Inventory/Items/Blueprints/Items/BaseItem_BP.BaseItem_BP_C|GetItemProps _asbase_item_bp))) (.MaxCount (Utilities|Struct|BreakItem (Variables|/Game/Inventory/Items/Blueprints/Items/BaseItem_BP.BaseItem_BP_C|GetItemProps _asbase_item_bp))) (.Icon (Utilities|Struct|BreakItem (Variables|/Game/Inventory/Items/Blueprints/Items/BaseItem_BP.BaseItem_BP_C|GetItemProps _asbase_item_bp))) "/Game/Inventory/Items/Blueprints/Items/In_Hand_Items/Food/F_Meat_BP.F_Meat_BP_C" false))
      (Utilities|FlowControl|DoOnce false) ; enters at Reset
    )))

(fn ConstructionScript
  (|CallParentFunction))