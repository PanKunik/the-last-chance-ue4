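; Placeable campfire item that burns wood fuel and lets the player roast items on an attachable grille, boil cauldron recipes or fire clay bars.
; A looping Fire timer drains burn time, scales the particles, hides wood meshes as fuel drops and drives Roasting, Boiling and Burning timers.
; Cooking timers pause when the fire dies.
; A widget HUD turns toward the player, shows fuel and burn time, and hides when not faced.
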(event Custom|Fire
  (bind _boilingitem (Variables|Default|GetBoilingItem))
  ;[1 1 1] FireUp Event
  (if (> (Variables|Burning|GetBurnTime) 0.0)
    (Utilities|FlowControl|Sequence
      (:then_0
        (Utilities|FlowControl|DoOnce false
          (:Completed
            (if (> (Variables|Burning|GetBurnTime) 24.0)
              (Variables|Burning|SetExpirationTime 12.0)
              (else
                (Variables|Burning|SetExpirationTime (/ (Variables|Burning|GetBurnTime) 2.0))))
            (if (Utilities|IsValid (Variables|Default|GetBurningItem))
              (bind _asbase_item_bp (Utilities|Casting|CastToBaseItem_BP (Variables|Default|GetBurningItem)))
              (Default|SetItemProps _asbase_item_bp (Utilities|Struct|MakeItem (.ID (Utilities|Struct|BreakItem (Variables|/Game/Inventory/Items/Blueprints/Items/BaseItem_BP.BaseItem_BP_C|GetItemProps _asbase_item_bp))) (.Name (Utilities|Struct|BreakItem (Variables|/Game/Inventory/Items/Blueprints/Items/BaseItem_BP.BaseItem_BP_C|GetItemProps _asbase_item_bp))) (.Stackable (Utilities|Struct|BreakItem (Variables|/Game/Inventory/Items/Blueprints/Items/BaseItem_BP.BaseItem_BP_C|GetItemProps _asbase_item_bp))) (.Type (Utilities|Struct|BreakItem (Variables|/Game/Inventory/Items/Blueprints/Items/BaseItem_BP.BaseItem_BP_C|GetItemProps _asbase_item_bp))) (.Count (Utilities|Struct|BreakItem (Variables|/Game/Inventory/Items/Blueprints/Items/BaseItem_BP.BaseItem_BP_C|GetItemProps _asbase_item_bp))) (.MaxCount (Utilities|Struct|BreakItem (Variables|/Game/Inventory/Items/Blueprints/Items/BaseItem_BP.BaseItem_BP_C|GetItemProps _asbase_item_bp))) (.Icon (Utilities|Struct|BreakItem (Variables|/Game/Inventory/Items/Blueprints/Items/BaseItem_BP.BaseItem_BP_C|GetItemProps _asbase_item_bp))) (.Class (Utilities|Struct|BreakItem (Variables|/Game/Inventory/Items/Blueprints/Items/BaseItem_BP.BaseItem_BP_C|GetItemProps _asbase_item_bp))) false))))))
      (:then_1
        (if (> (Variables|Burning|GetBurnTime) (Variables|Burning|GetExpirationTime))
          (Transformation|SetWorldScale3D (Variables|Default|GetFire_PS) (Math|Vector|MakeVector (Math|Interpolation|FInterptoConstant (Variables|Burning|GetScale) 3.0 (Variables|Burning|GetTimeTick) 0.25) (Math|Interpolation|FInterptoConstant (Variables|Burning|GetScale) 3.0 (Variables|Burning|GetTimeTick) 0.25) (Math|Interpolation|FInterptoConstant (Variables|Burning|GetScale) 3.0 (Variables|Burning|GetTimeTick) 0.25)))
          (Variables|Burning|SetScale (Math|Interpolation|FInterptoConstant (Variables|Burning|GetScale) 3.0 (Variables|Burning|GetTimeTick) 0.25))
          (Variables|Burning|SetBurnTime (Math|Interpolation|FInterptoConstant (Variables|Burning|GetBurnTime) 0.0 (Variables|Burning|GetTimeTick) 1.0))
          (Variables|Burning|SetElapsed (Math|Interpolation|FInterptoConstant (Variables|Burning|GetElapsed) 6e+01 (Variables|Burning|GetTimeTick) 1.0))
          (else
            (Transformation|SetWorldScale3D (Variables|Default|GetFire_PS) (Math|Vector|MakeVector (Math|Interpolation|FInterptoConstant (Variables|Burning|GetScale) 0.0 (Variables|Burning|GetTimeTick) 0.25) (Math|Interpolation|FInterptoConstant (Variables|Burning|GetScale) 0.0 (Variables|Burning|GetTimeTick) 0.25) (Math|Interpolation|FInterptoConstant (Variables|Burning|GetScale) 0.0 (Variables|Burning|GetTimeTick) 0.25)))
            (Variables|Burning|SetScale (Math|Interpolation|FInterptoConstant (Variables|Burning|GetScale) 0.0 (Variables|Burning|GetTimeTick) 0.25))
            (Variables|Burning|SetBurnTime (Math|Interpolation|FInterptoConstant (Variables|Burning|GetBurnTime) 0.0 (Variables|Burning|GetTimeTick) 1.0))
            (Variables|Burning|SetElapsed (Math|Interpolation|FInterptoConstant (Variables|Burning|GetElapsed) 6e+01 (Variables|Burning|GetTimeTick) 1.0)))))
      (:then_2
        (if (> (Variables|Fuel|GetFuelFill) 0)
          (if (>= (Variables|Burning|GetElapsed) 2e+01)
            (Variables|Burning|SetElapsed (- (Variables|Burning|GetElapsed) 2e+01))
            (CallFunction|HideWood)
            (Variables|Fuel|SetFuelFill (- (Variables|Fuel|GetFuelFill) 1)))))
      (:then_3
        (if (Variables|Default|GetCanItemBeRoasted)
          (if (Utilities|Time|IsTimerActivebyHandle (Variables|Default|GetRoasting_TH))
            (Utilities|Time|UnpauseTimerbyHandle (Variables|Default|GetRoasting_TH))
            (else
              (bind _returnvalue (Utilities|Time|SetTimerbyFunctionName self "Roasting" (Variables|Burning|GetTimeTick) true))
              (Variables|Default|SetRoasting_TH _returnvalue)))))
      (:then_4
        (if (Variables|Default|GetCanItemBeBurned)
          (if (Utilities|Time|IsTimerActivebyHandle (Variables|Default|GetBurningItem_TH))
            (Utilities|Time|UnpauseTimerbyHandle (Variables|Default|GetBurningItem_TH))
            (else
              (bind _returnvalue_2 (Utilities|Time|SetTimerbyFunctionName self "Burning" (Variables|Burning|GetTimeTick) true))
              (Variables|Default|SetBurningItem_TH _returnvalue_2)))))
      (:then_5
        (if (and (Utilities|IsValid _boilingitem) (not (Variables|Default|GetCanItemBeBoiled)))
          (bind _ascauldron_bp (Utilities|Casting|CastToCauldron_BP _boilingitem))
          (if (not (Variables|/Game/Inventory/Items/Blueprints/Items/In_Hand_Items/Utilities/Cauldron_BP.Cauldron_BP_C|GetIsRecipeReady? _ascauldron_bp))
            (Default|CheckRecipe _ascauldron_bp)
            (if (> (.BolingTime (Utilities|Struct|BreakSTR_Boiling (Variables|/Game/Inventory/Items/Blueprints/Items/In_Hand_Items/Utilities/Cauldron_BP.Cauldron_BP_C|GetActiveRecipe _ascauldron_bp))) 0.0)
              (Variables|Default|SetCanItemBeBoiled true)
              (Variables|Burning|SetBoilingTime (.BolingTime (Utilities|Struct|BreakSTR_Boiling (Variables|/Game/Inventory/Items/Blueprints/Items/In_Hand_Items/Utilities/Cauldron_BP.Cauldron_BP_C|GetActiveRecipe _ascauldron_bp))))))))
      (:then_6
        (if (Variables|Default|GetCanItemBeBoiled)
          (if (Utilities|Time|IsTimerActivebyHandle (Variables|Default|GetBoiling_TH))
            (Utilities|Time|UnpauseTimerbyHandle (Variables|Default|GetBoiling_TH))
            (else
              (bind _returnvalue_3 (Utilities|Time|SetTimerbyFunctionName self "Boiling" (Variables|Burning|GetTimeTick) true))
              (Variables|Default|SetBoiling_TH _returnvalue_3))))))
    (else
      (Utilities|Time|ClearandInvalidateTimerbyHandle (Variables|Burning|GetBurning_TH))
      (Components|Activation|SetActive (Variables|Default|GetFire_PS) false false)
      (Variables|Burning|SetScale 0.0)
      (Rendering|SetVisibility (Variables|Default|GetItemMesh) false false)
      (Variables|Burning|SetBurningTime 0.0)
      (Variables|Burning|SetElapsed 0.0)
      (Variables|Fuel|SetFuelFill 0)
      (Utilities|FlowControl|Sequence
        (:then_0
          (CallFunction|ResetFiringDoOnce))
        (:then_1
          (if (Utilities|Time|IsTimerActivebyHandle (Variables|Default|GetBurningItem_TH))
            (Utilities|Time|PauseTimerbyHandle (Variables|Default|GetBurningItem_TH))))
        (:then_2
          (if (Utilities|Time|IsTimerActivebyHandle (Variables|Default|GetRoasting_TH))
            (Utilities|Time|PauseTimerbyHandle (Variables|Default|GetRoasting_TH))))
        (:then_3
          (if (and (Utilities|IsValid (Variables|Default|GetBurningItem)) (not (Variables|Default|GetCanItemBeBurned)))
            (bind _asbase_item_bp_2 (Utilities|Casting|CastToBaseItem_BP (Variables|Default|GetBurningItem)))
            (Default|SetItemProps _asbase_item_bp_2 (Utilities|Struct|MakeItem (.ID (Utilities|Struct|BreakItem (Variables|/Game/Inventory/Items/Blueprints/Items/BaseItem_BP.BaseItem_BP_C|GetItemProps _asbase_item_bp_2))) (.Name (Utilities|Struct|BreakItem (Variables|/Game/Inventory/Items/Blueprints/Items/BaseItem_BP.BaseItem_BP_C|GetItemProps _asbase_item_bp_2))) (.Stackable (Utilities|Struct|BreakItem (Variables|/Game/Inventory/Items/Blueprints/Items/BaseItem_BP.BaseItem_BP_C|GetItemProps _asbase_item_bp_2))) (.Type (Utilities|Struct|BreakItem (Variables|/Game/Inventory/Items/Blueprints/Items/BaseItem_BP.BaseItem_BP_C|GetItemProps _asbase_item_bp_2))) (.Count (Utilities|Struct|BreakItem (Variables|/Game/Inventory/Items/Blueprints/Items/BaseItem_BP.BaseItem_BP_C|GetItemProps _asbase_item_bp_2))) (.MaxCount (Utilities|Struct|BreakItem (Variables|/Game/Inventory/Items/Blueprints/Items/BaseItem_BP.BaseItem_BP_C|GetItemProps _asbase_item_bp_2))) (.Icon (Utilities|Struct|BreakItem (Variables|/Game/Inventory/Items/Blueprints/Items/BaseItem_BP.BaseItem_BP_C|GetItemProps _asbase_item_bp_2))) (.Class (Utilities|Struct|BreakItem (Variables|/Game/Inventory/Items/Blueprints/Items/BaseItem_BP.BaseItem_BP_C|GetItemProps _asbase_item_bp_2)))))))
        (:then_4
          (if (Utilities|Time|IsTimerActivebyHandle (Variables|Default|GetBoiling_TH))
            (Utilities|Time|PauseTimerbyHandle (Variables|Default|GetBoiling_TH))))))))

(event Custom|HideWood
  ;[1 1 1] Event HideCoal -> When they burn
  (switch int (- (Variables|Fuel|GetFuelFill) 1)
    (:0
      (Rendering|SetVisibility (Variables|Default|GetItemMesh) false false))
    (:1
      (Rendering|SetVisibility (Variables|Default|GetStaticMesh) false false))
    (:2
      (Rendering|SetVisibility (Variables|Default|GetStaticMesh1) false false))
    (:3
      (Rendering|SetVisibility (Variables|Default|GetStaticMesh2) false false))
    (:4
      (Rendering|SetVisibility (Variables|Default|GetStaticMesh3) false false))
    (:5
      (Rendering|SetVisibility (Variables|Default|GetStaticMesh4) false false))))

(event Custom|RotateHUD
  (bind _returnvalue (Game|GetPlayerCharacter 0))
  (bind _campfire_hud (Variables|Default|GetCampfire_HUD))
  ;[1 1 1] Rotating HUD to players rotation (Timer)
  (Utilities|IsValid _returnvalue
    (:Is%20Valid
      (Transformation|SetWorldRotation _campfire_hud (Math|Rotator|MakeRotator 0.0 0.0 (.Yaw (Math|Rotator|BreakRotator (Math|Rotator|FindLookatRotation (Transformation|GetWorldLocation (Variables|Default|GetCampfire_HUD)) (Transformation|GetWorldLocation (Variables|/Script/Engine.Character|GetCapsuleComponent _returnvalue)))))) false false)
      (bind _asumg_bw_small_campfire_hud (Utilities|Casting|CastToUMG_BW_SmallCampfireHUD (UserInterface|GetUserWidgetObject _campfire_hud)))
      (Variables|/Game/Inventory/HUD/ItemsHUD/UMG_BW_SmallCampfireHUD.UMG_BW_SmallCampfireHUD_C|SetHUD_WoodFuel _asumg_bw_small_campfire_hud (Utilities|Text|ToText(String) (Utilities|String|Append (Utilities|String|ToString(Integer) (Variables|Fuel|GetFuelFill)) "/6")))
      (Variables|/Game/Inventory/HUD/ItemsHUD/UMG_BW_SmallCampfireHUD.UMG_BW_SmallCampfireHUD_C|SetHUD_BurnTime _asumg_bw_small_campfire_hud (Utilities|Text|ToText(String) (Utilities|String|Append (Utilities|String|ToString(Integer) (Math|Float|Round (Variables|Burning|GetBurnTime))) " s")))
      (Variables|/Game/Inventory/HUD/ItemsHUD/UMG_BW_SmallCampfireHUD.UMG_BW_SmallCampfireHUD_C|SetHUD_Name _asumg_bw_small_campfire_hud (Utilities|Text|ToText(String) (.Name (Utilities|Struct|BreakItem (Variables|Default|GetItemProps)))))
      (Variables|/Game/Inventory/HUD/ItemsHUD/UMG_BW_SmallCampfireHUD.UMG_BW_SmallCampfireHUD_C|SetHUD_ProgressBarValue _asumg_bw_small_campfire_hud (/ (Variables|Burning|GetBurnTime) (Variables|Burning|GetMaxBurnTime))))))

(event Custom|Roasting
  ;[1 1 1] Event RoastItem
  (bind _output_get (Variables|Burning|SetRoastTime (Math|Interpolation|FInterptoConstant (Variables|Burning|GetRoastTime) 0.0 (Variables|Burning|GetTimeTick) 1.0)))
  (if (not (> _output_get 0.0))
    (Utilities|FlowControl|DoOnce false
      (:Completed
        (bind _asbase_item_bp (Utilities|Casting|CastToBaseItem_BP (Variables|Default|GetRoastingItem)))
        (bind _roasteditem (Default|ChangeRoastedItem _asbase_item_bp))
        (bind _returnvalue (Game|SpawnActorfromClass _roasteditem (Transformation|GetActorTransform (Variables|Default|GetRoastingItem)) "Undefined" 0 0))
        (Actor|DestroyActor (Variables|Default|GetRoastingItem))
        (Variables|Default|SetRoastingItem _returnvalue)
        (Utilities|Time|ClearandInvalidateTimerbyHandle (Variables|Default|GetRoasting_TH))
        (Variables|Default|SetCanItemBeRoasted false)))))

(event Custom|ResetFiringDoOnce
  ;[1 1 1] FireUp Event
  (Utilities|FlowControl|DoOnce false) ; enters at Reset
)

(event Custom|Burning
  (bind _output_get (Variables|Burning|SetBurningTime (Math|Interpolation|FInterptoConstant (Variables|Burning|GetBurningTime) 0.0 (Variables|Burning|GetTimeTick) 1.0)))
  (if (not (> _output_get 0.0))
    (Utilities|FlowControl|DoOnce false
      (:Completed
        (Class|UsingItemsInterface|ChangeBurnedItem(Message) (Variables|Default|GetBurningItem))
        (Variables|Default|SetCanItemBeBurned false)))))

(event Custom|Boiling
  (bind _output_get (Variables|Burning|SetBoilingTime (Math|Interpolation|FInterptoConstant (Variables|Burning|GetBoilingTime) 0.0 (Variables|Burning|GetTimeTick) 1.0)))
  (if (not (> _output_get 0.0))
    (Utilities|FlowControl|Sequence
      (:then_0
        (Utilities|FlowControl|DoOnce false :!label _label
          (:Completed
            (bind _ascauldron_bp (Utilities|Casting|CastToCauldron_BP (Variables|Default|GetBoilingItem)))
            (Default|Ready _ascauldron_bp)
            (Variables|Default|SetCanItemBeBoiled false))))
      (:then_1
        (if (Variables|Default|GetCanItemBeBoiled)
          (goto _label Reset))))))

(event Custom|CheckingFacing
  (bind _asfirst_person_character (Utilities|Casting|CastToFirstPersonCharacter (Game|GetPlayerCharacter 0)))
  (if (not (== (Variables|/Game/FirstPersonBP/Blueprints/FirstPersonCharacter.FirstPersonCharacter_C|GetFacingActor _asfirst_person_character) self))
    (CallFunction|HideHUD)
    (Utilities|Time|ClearandInvalidateTimerbyHandle (Variables|Default|GetCheckingFacing_TH))))

(event EventBeginPlay
  (|CallParentFunction)
  ;[1 1 1] Event BeginPlay -> Attach Wood (Fuel) to campfire
  (Rendering|SetVisibility (Variables|Default|GetCampfire_HUD) false false)
  (Variables|Burning|SetMaxBurnTime 1.2e+02)
  (Variables|Burning|SetBurnTime 1.2e+02)
  (Variables|Fuel|SetFuelFill 6)
  (Variables|Default|SetCanItemBeRoasted false)
  (Utilities|Time|SetTimerbyFunctionName self "RotateHUD" 0.01 true))

(event EventHideHUD
  (Utilities|FlowControl|Sequence
    (:then_0
      (Utilities|FlowControl|DoOnce false) ; enters at Reset
    )
    (:then_1
      (Utilities|FlowControl|DoOnce true
        (:Completed
          (bind _asumg_bw_small_campfire_hud (Utilities|Casting|CastToUMG_BW_SmallCampfireHUD (UserInterface|GetUserWidgetObject (Variables|Default|GetCampfire_HUD))))
          (UserInterface|Animation|PlayAnimation _asumg_bw_small_campfire_hud (Variables|/Game/Inventory/HUD/ItemsHUD/UMG_BW_SmallCampfireHUD.UMG_BW_SmallCampfireHUD_C|GetFadeIn _asumg_bw_small_campfire_hud) (Class|UserWidget|GetAnimationCurrentTime _asumg_bw_small_campfire_hud (Variables|/Game/Inventory/HUD/ItemsHUD/UMG_BW_SmallCampfireHUD.UMG_BW_SmallCampfireHUD_C|GetFadeIn _asumg_bw_small_campfire_hud)) 1 "Reverse" 1.0))))))

(event EventPutItem
  (params (Class :type Actor%20Class%20Reference))
  (if (Math|Boolean|ANDBoolean (not (Utilities|IsValid (Variables|Default|GetRoastingItem))) (not (Utilities|IsValid (Variables|Default|GetBoilingItem))) (not (Utilities|IsValid (Variables|Default|GetBurningItem))))
    (if (== Class "/Game/Inventory/Items/Blueprints/Items/In_Hand_Items/Utilities/Cauldron_BP.Cauldron_BP_C")
      (bind _returnvalue (Game|SpawnActorfromClass Class (Math|Transform|MakeTransform "0, 0, 0") "Undefined" self 0))
      (bind _output_get (Variables|Default|SetBoilingItem _returnvalue))
      (CallFunction|RemoveItemonUse)
      (Transformation|AddActorLocalOffset _output_get (- (Transformation|GetSocketLocation (Variables|Default|GetItemMesh) "BoilingSocket") (Transformation|GetActorLocation)) false false)
      (Transformation|AttachActorToActor (Variables|Default|GetBoilingItem) self "BoilingSocket" "KeepRelative" "KeepWorld" "KeepRelative" true)
      (Variables|Default|SetCanItemBeBoiled false)
      (bind _ascauldron_bp (Utilities|Casting|CastToCauldron_BP (Variables|Default|GetBoilingItem)))
      (Default|SetItemProps _ascauldron_bp (Utilities|Struct|MakeItem (.ID (Utilities|Struct|BreakItem (Variables|/Game/Inventory/Items/Blueprints/Items/BaseItem_BP.BaseItem_BP_C|GetItemProps _ascauldron_bp))) (.Name (Utilities|Struct|BreakItem (Variables|/Game/Inventory/Items/Blueprints/Items/BaseItem_BP.BaseItem_BP_C|GetItemProps _ascauldron_bp))) (.Stackable (Utilities|Struct|BreakItem (Variables|/Game/Inventory/Items/Blueprints/Items/BaseItem_BP.BaseItem_BP_C|GetItemProps _ascauldron_bp))) (.Type (Utilities|Struct|BreakItem (Variables|/Game/Inventory/Items/Blueprints/Items/BaseItem_BP.BaseItem_BP_C|GetItemProps _ascauldron_bp))) (.Count (Utilities|Struct|BreakItem (Variables|/Game/Inventory/Items/Blueprints/Items/BaseItem_BP.BaseItem_BP_C|GetItemProps _ascauldron_bp))) (.MaxCount (Utilities|Struct|BreakItem (Variables|/Game/Inventory/Items/Blueprints/Items/BaseItem_BP.BaseItem_BP_C|GetItemProps _ascauldron_bp))) (.Icon (Utilities|Struct|BreakItem (Variables|/Game/Inventory/Items/Blueprints/Items/BaseItem_BP.BaseItem_BP_C|GetItemProps _ascauldron_bp))) (.Class (Utilities|Struct|BreakItem (Variables|/Game/Inventory/Items/Blueprints/Items/BaseItem_BP.BaseItem_BP_C|GetItemProps _ascauldron_bp))) false))
      (elif (== Class "/Game/Inventory/Items/Blueprints/Items/Resources/ClayBar_BP.ClayBar_BP_C")
        (bind _returnvalue_2 (Game|SpawnActorfromClass Class (Math|Transform|MakeTransform "0, 0, 0") "Undefined" self 0))
        (bind _output_get_2 (Variables|Default|SetBurningItem _returnvalue_2))
        (CallFunction|RemoveItemonUse)
        (Transformation|AddActorLocalOffset _output_get_2 (- (Transformation|GetSocketLocation (Variables|Default|GetItemMesh) "BoilingSocket") (Transformation|GetActorLocation)) false false)
        (Transformation|AttachActorToActor (Variables|Default|GetBurningItem) self "BoilingSocket" "KeepRelative" "KeepWorld" "KeepRelative" true)
        (Variables|Default|SetCanItemBeBurned true)
        (Variables|Burning|SetBurningTime 3e+01)
        (bind _asbase_item_bp (Utilities|Casting|CastToBaseItem_BP (Variables|Default|GetBurningItem)))
        (Default|SetItemProps _asbase_item_bp (Utilities|Struct|MakeItem (.ID (Utilities|Struct|BreakItem (Variables|/Game/Inventory/Items/Blueprints/Items/BaseItem_BP.BaseItem_BP_C|GetItemProps _asbase_item_bp))) (.Name (Utilities|Struct|BreakItem (Variables|/Game/Inventory/Items/Blueprints/Items/BaseItem_BP.BaseItem_BP_C|GetItemProps _asbase_item_bp))) (.Stackable (Utilities|Struct|BreakItem (Variables|/Game/Inventory/Items/Blueprints/Items/BaseItem_BP.BaseItem_BP_C|GetItemProps _asbase_item_bp))) (.Type (Utilities|Struct|BreakItem (Variables|/Game/Inventory/Items/Blueprints/Items/BaseItem_BP.BaseItem_BP_C|GetItemProps _asbase_item_bp))) (.Count (Utilities|Struct|BreakItem (Variables|/Game/Inventory/Items/Blueprints/Items/BaseItem_BP.BaseItem_BP_C|GetItemProps _asbase_item_bp))) (.MaxCount (Utilities|Struct|BreakItem (Variables|/Game/Inventory/Items/Blueprints/Items/BaseItem_BP.BaseItem_BP_C|GetItemProps _asbase_item_bp))) (.Icon (Utilities|Struct|BreakItem (Variables|/Game/Inventory/Items/Blueprints/Items/BaseItem_BP.BaseItem_BP_C|GetItemProps _asbase_item_bp))) (.Class (Utilities|Struct|BreakItem (Variables|/Game/Inventory/Items/Blueprints/Items/BaseItem_BP.BaseItem_BP_C|GetItemProps _asbase_item_bp))) false))
        (Utilities|FlowControl|DoOnce false) ; enters at Reset
      ))))

(event EventAddFuel
  (params (FuelClass :type Actor%20Class%20Reference))
  (bind _fuelitems (Variables|Fuel|GetFuelItems))
  (bind (_fuelobject _fuelcapacity _burntime) (Utilities|Struct|BreakSTR_FuelItem _fuelitems))
  ;[1 1 1] Event AddFuel -> When adding coals
  (Utilities|FlowControl|Sequence
    (:then_0
      (if (== FuelClass _fuelobject)
        (if (< (+ (Variables|Fuel|GetFuelFill) _fuelcapacity) 7)
          (CallFunction|RemoveItemonUse)
          (Variables|Fuel|SetFuelFill (+ (Variables|Fuel|GetFuelFill) _fuelcapacity))
          (Variables|Burning|SetBurnTime (+ (Variables|Burning|GetBurnTime) _burntime))
          (switch int (- (Variables|Fuel|GetFuelFill) 1)
            (:0
              (Rendering|SetVisibility (Variables|Default|GetItemMesh) true false))
            (:1
              (Rendering|SetVisibility (Variables|Default|GetStaticMesh) true false))
            (:2
              (Rendering|SetVisibility (Variables|Default|GetStaticMesh1) true false))
            (:3
              (Rendering|SetVisibility (Variables|Default|GetStaticMesh2) true false))
            (:4
              (Rendering|SetVisibility (Variables|Default|GetStaticMesh3) true false))
            (:5
              (Rendering|SetVisibility (Variables|Default|GetStaticMesh4) true false))))))
    (:then_1
      (CallFunction|ResetFiringDoOnce))))

(event EventIgnite
  ;[1 1 1] Event Ignite
  (Variables|Burning|SetTimeTick 0.05)
  (if (> (Variables|Burning|GetBurnTime) 0.0)
    (if (not (Utilities|Time|IsTimerActivebyHandle (Variables|Burning|GetBurning_TH)))
      (bind _returnvalue (Utilities|Time|SetTimerbyFunctionName self "Fire" (Variables|Burning|GetTimeTick) true))
      (Variables|Burning|SetBurning_TH _returnvalue)
      (Components|Activation|SetActive (Variables|Default|GetFire_PS) true true))))

(event EventShowHUD
  (Utilities|FlowControl|Sequence
    (:then_0
      (Utilities|FlowControl|DoOnce false
        (:Completed
          (Rendering|SetVisibility (Variables|Default|GetCampfire_HUD) true false)
          (bind _returnvalue (Utilities|Time|SetTimerbyFunctionName 0 "CheckingFacing" (Variables|Burning|GetTimeTick) true))
          (Variables|Default|SetCheckingFacing_TH _returnvalue)
          (bind _asumg_bw_small_campfire_hud (Utilities|Casting|CastToUMG_BW_SmallCampfireHUD (UserInterface|GetUserWidgetObject (Variables|Default|GetCampfire_HUD))))
          (UserInterface|Animation|PlayAnimation _asumg_bw_small_campfire_hud (Variables|/Game/Inventory/HUD/ItemsHUD/UMG_BW_SmallCampfireHUD.UMG_BW_SmallCampfireHUD_C|GetFadeIn _asumg_bw_small_campfire_hud) (Class|UserWidget|GetAnimationCurrentTime _asumg_bw_small_campfire_hud (Variables|/Game/Inventory/HUD/ItemsHUD/UMG_BW_SmallCampfireHUD.UMG_BW_SmallCampfireHUD_C|GetFadeIn _asumg_bw_small_campfire_hud)) 1 "Forward" 1.0))))
    (:then_1
      (Utilities|FlowControl|DoOnce true) ; enters at Reset
    )))

(event EventRemoveItemonUse
  (bind _asfirst_person_character (Utilities|Casting|CastToFirstPersonCharacter (Game|GetPlayerCharacter 0)))
  (Class|RemoveItem|RemoveOneItemCount(Message) (Variables|/Game/FirstPersonBP/Blueprints/FirstPersonCharacter.FirstPersonCharacter_C|GetEquipedItem _asfirst_person_character))
  (Default|UpdateInventoryHUD _asfirst_person_character))

(event EventRoastItem
  (params (Item :type Actor%20Class%20Reference))
  ;[1 1 1] Event RoastItem
  (if (Variables|Default|GetIsGrilleAttached)
    (if (Math|Boolean|ANDBoolean (not (Utilities|IsValid (Variables|Default|GetRoastingItem))) (not (Utilities|IsValid (Variables|Default|GetBoilingItem))) (not (Utilities|IsValid (Variables|Default|GetBurningItem))))
      (Variables|Default|SetCanItemBeRoasted true)
      (Variables|Burning|SetRoastTime 1.1e+02)
      (bind _returnvalue (Game|SpawnActorfromClass Item (Math|Transform|MakeTransform "0, 0, 0") "Undefined" self 0))
      (bind _output_get (Variables|Default|SetRoastingItem _returnvalue))
      (CallFunction|RemoveItemonUse)
      (Transformation|AddActorLocalOffset _output_get (- (Transformation|GetSocketLocation (Variables|Default|GetItemMesh) "RoastingSocket") (Transformation|GetActorLocation)) false false)
      (Transformation|SetActorRotation (Variables|Default|GetRoastingItem) (Variables|Default|GetGrilleRotation))
      (Transformation|AttachActorToActor (Variables|Default|GetRoastingItem) self "RoastingSocket" "KeepRelative" "KeepWorld" "KeepRelative" true)
      (bind _asbase_item_bp (Utilities|Casting|CastToBaseItem_BP (Variables|Default|GetRoastingItem)))
      (Default|SetItemProps _asbase_item_bp (Utilities|Struct|MakeItem (.ID (Utilities|Struct|BreakItem (Variables|/Game/Inventory/Items/Blueprints/Items/BaseItem_BP.BaseItem_BP_C|GetItemProps _asbase_item_bp))) (.Name (Utilities|Struct|BreakItem (Variables|/Game/Inventory/Items/Blueprints/Items/BaseItem_BP.BaseItem_BP_C|GetItemProps _asbase_item_bp))) (.Stackable (Utilities|Struct|BreakItem (Variables|/Game/Inventory/Items/Blueprints/Items/BaseItem_BP.BaseItem_BP_C|GetItemProps _asbase_item_bp))) (.Type (Utilities|Struct|BreakItem (Variables|/Game/Inventory/Items/Blueprints/Items/BaseItem_BP.BaseItem_BP_C|GetItemProps _asbase_item_bp))) (.Count (Utilities|Struct|BreakItem (Variables|/Game/Inventory/Items/Blueprints/Items/BaseItem_BP.BaseItem_BP_C|GetItemProps _asbase_item_bp))) (.MaxCount (Utilities|Struct|BreakItem (Variables|/Game/Inventory/Items/Blueprints/Items/BaseItem_BP.BaseItem_BP_C|GetItemProps _asbase_item_bp))) (.Icon (Utilities|Struct|BreakItem (Variables|/Game/Inventory/Items/Blueprints/Items/BaseItem_BP.BaseItem_BP_C|GetItemProps _asbase_item_bp))) "/Game/Inventory/Items/Blueprints/Items/In_Hand_Items/Food/F_Meat_BP.F_Meat_BP_C" false))
      (Utilities|FlowControl|DoOnce false) ; enters at Reset
    )))

(event EventAttachGrille
  ;[1 1 1] Event AttachGrille
  (Utilities|FlowControl|DoOnce false
    (:Completed
      (bind _returnvalue (Game|SpawnActorfromClass "/Game/Inventory/Items/Blueprints/Items/In_Hand_Items/Utilities/CampfireGrille_BP.CampfireGrille_BP_C" (Math|Transform|MakeTransform "0, 0, 0") "Undefined" 0 0))
      (Transformation|AttachActorToActor _returnvalue self "CampfireGrille" "KeepRelative" "KeepWorld" "KeepRelative" true)
      (bind _output_get (Variables|Default|SetGrilleRotation (Math|Rotator|MakeRotator 0.0 0.0 (+ (.Yaw (Math|Rotator|BreakRotator (Transformation|GetActorRotation (Game|GetPlayerCharacter 0)))) 9e+01))))
      (Transformation|SetActorRotation _returnvalue _output_get)
      (Variables|Default|SetIsGrilleAttached true)
      (Transformation|AddLocalOffset (Variables|Default|GetCampfire_HUD) "0, 0,50.000000" false false)
      (Default|SetItemProps _returnvalue (Utilities|Struct|MakeItem (.ID (Utilities|Struct|BreakItem (Variables|/Game/Inventory/Items/Blueprints/Items/BaseItem_BP.BaseItem_BP_C|GetItemProps _returnvalue))) (.Name (Utilities|Struct|BreakItem (Variables|/Game/Inventory/Items/Blueprints/Items/BaseItem_BP.BaseItem_BP_C|GetItemProps _returnvalue))) (.Stackable (Utilities|Struct|BreakItem (Variables|/Game/Inventory/Items/Blueprints/Items/BaseItem_BP.BaseItem_BP_C|GetItemProps _returnvalue))) (.Type (Utilities|Struct|BreakItem (Variables|/Game/Inventory/Items/Blueprints/Items/BaseItem_BP.BaseItem_BP_C|GetItemProps _returnvalue))) (.Count (Utilities|Struct|BreakItem (Variables|/Game/Inventory/Items/Blueprints/Items/BaseItem_BP.BaseItem_BP_C|GetItemProps _returnvalue))) (.MaxCount (Utilities|Struct|BreakItem (Variables|/Game/Inventory/Items/Blueprints/Items/BaseItem_BP.BaseItem_BP_C|GetItemProps _returnvalue))) (.Icon (Utilities|Struct|BreakItem (Variables|/Game/Inventory/Items/Blueprints/Items/BaseItem_BP.BaseItem_BP_C|GetItemProps _returnvalue))) (.Class (Utilities|Struct|BreakItem (Variables|/Game/Inventory/Items/Blueprints/Items/BaseItem_BP.BaseItem_BP_C|GetItemProps _returnvalue))) false))
      (CallFunction|RemoveItemonUse))))

(event Collision|EventActorBeginOverlap
  (params (OtherActor :type Actor%20Object%20Reference))
  (|CallParentFunction OtherActor) ; This node is disabled and will not be called.\nDrag off pins to build functionality.
)

(fn ConstructionScript
  (|CallParentFunction))