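; Furnace utility item that burns fuel to melt or burn materials placed inside, with a floating fuel HUD that turns toward the player.
; AddFuel and PutItem spawn capacity-limited item actors, briefly enabling their physics through a CountDown timer.
; Ignite starts Fire, which scales flames, consumes fuel and counts down each material before sending it ChangeBurnedItemMessage.
; Looping timers drive all updates instead of Tick, with resettable DoOnce gates.
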(event Custom|Fire
  (bind _fuel (Variables|Fuel|GetFuel))
  ;[1 1 1] Event Fire -> When ignited
  (Utilities|FlowControl|Sequence
    (:then_0
      (Utilities|FlowControl|DoOnce false
        (:Completed
          (if (> (Variables|Burning|GetBurnTime) 4e+01)
            (Variables|Burning|SetExpiringTime 2e+01)
            (else
              (Variables|Burning|SetExpiringTime (/ (Variables|Burning|GetBurnTime) 2.0)))))))
    (:then_1
      (Utilities|FlowControl|DoOnce false
        (:Completed
          (Variables|Fuel|SetElapsingActor (Utilities|Array|Get(acopy) _fuel (- (Utilities|Array|Length _fuel) 1))))))
    (:then_2
      (Variables|Burning|SetBurnTime (Math|Interpolation|FInterptoConstant (Variables|Burning|GetBurnTime) 0.0 (Variables|Burning|GetTimeTick) 1.0))
      (if (or (> (Variables|Burning|GetBurnTime) 0.0) (> (Utilities|Array|Length (Variables|Fuel|GetFuel)) 0))
        (Utilities|FlowControl|Sequence
          (:then_0
            (if (> (Variables|Burning|GetBurnTime) (Variables|Burning|GetExpiringTime))
              (bind _output_get (Variables|Burning|SetScale (Math|Interpolation|FInterptoConstant (Variables|Burning|GetScale) 5.0 (Variables|Burning|GetTimeTick) 0.25)))
              (Transformation|SetRelativeScale3D (Variables|Default|GetParticleSystem) (Math|Vector|MakeVector _output_get _output_get _output_get))
              (else
                (bind _output_get_2 (Variables|Burning|SetScale (Math|Interpolation|FInterptoConstant (Variables|Burning|GetScale) 0.1 (Variables|Burning|GetTimeTick) 0.25)))
                (Transformation|SetRelativeScale3D (Variables|Default|GetParticleSystem) (Math|Vector|MakeVector _output_get_2 _output_get_2 _output_get_2))))
            (bind _output_get_3 (Variables|Burning|SetElapsed (Math|Interpolation|FInterptoConstant (Variables|Burning|GetElapsed) 6e+01 (Variables|Burning|GetTimeTick) 1.0)))
            (if (>= _output_get_3 5.0)
              (for _array_element (Variables|Fuel|GetFuelItems)
                (if (== (.FuelObject (Utilities|Struct|BreakSTR_FuelItem _array_element)) (Utilities|GetClass (Variables|Fuel|GetElapsingActor)))
                  (if (>= (Variables|Burning|GetElapsed) (.BurnTime (Utilities|Struct|BreakSTR_FuelItem _array_element)))
                    (Variables|Burning|SetElapsed (- (Variables|Burning|GetElapsed) (.BurnTime (Utilities|Struct|BreakSTR_FuelItem _array_element))))
                    (Utilities|Array|RemoveItem (Variables|Fuel|GetFuel) (Variables|Fuel|GetElapsingActor))
                    (Actor|DestroyActor (Variables|Fuel|GetElapsingActor))
                    (Variables|Fuel|SetFuelFill (- (Variables|Fuel|GetFuelFill) (.FuelCapacity (Utilities|Struct|BreakSTR_FuelItem _array_element))))
                    (CallFunction|ResetElapsingDoOnce)
                    (Variables|Fuel|SetTimer 3.0)
                    (if (Utilities|Time|IsTimerActivebyHandle (Variables|Fuel|GetCountDown_TH))
                      (CallFunction|ResetPhysicsDoOnce)
                      (Utilities|Time|ClearandInvalidateTimerbyHandle (Variables|Fuel|GetCountDown_TH)))
                    (bind _returnvalue (Utilities|Time|SetTimerbyFunctionName self "CountDown" (Variables|Burning|GetTimeTick) true))
                    (Variables|Fuel|SetCountDown_TH _returnvalue))))))
          (:then_1
            (if (> (Variables|Materials|GetMaterialFill) 0)
              (for (_array_element_2 _array_index) (Variables|Materials|GetMaterialsBurning)
                (bind _output_get_4 (Variables|Default|SetRemainingTimeHelper (.RemainingTime (Utilities|Struct|BreakSTR_BurningItem _array_element_2))))
                (if (> _output_get_4 0.0)
                  (Utilities|Array|SetArrayElem (Variables|Materials|GetMaterialsBurning) _array_index (Utilities|Struct|MakeSTR_BurningItem (.MaterialObject (Utilities|Struct|BreakSTR_BurningItem _array_element_2)) (Math|Interpolation|FInterptoConstant _output_get_4 0.0 (Variables|Burning|GetTimeTick) 1.0) false))
                  (elif (not (.Burned (Utilities|Struct|BreakSTR_BurningItem _array_element_2)))
                    (Class|UsingItemsInterface|ChangeBurnedItem(Message) (.MaterialObject (Utilities|Struct|BreakSTR_BurningItem _array_element_2)))
                    (Utilities|Array|SetArrayElem (Variables|Materials|GetMaterialsBurning) _array_index (Utilities|Struct|MakeSTR_BurningItem (.MaterialObject (Utilities|Struct|BreakSTR_BurningItem _array_element_2)) 0.0 true))))))))
        (else
          (for _array_element_3 (Variables|Materials|GetMaterialsBurning)
            (bind _asbase_item_bp (Utilities|Casting|CastToBaseItem_BP (.MaterialObject (Utilities|Struct|BreakSTR_BurningItem _array_element_3))))
            (Variables|/Game/Inventory/Items/Blueprints/Items/BaseItem_BP.BaseItem_BP_C|SetItemProps _asbase_item_bp (Utilities|Struct|MakeItem (.ID (Utilities|Struct|BreakItem (Variables|/Game/Inventory/Items/Blueprints/Items/BaseItem_BP.BaseItem_BP_C|GetItemProps _asbase_item_bp))) (.Name (Utilities|Struct|BreakItem (Variables|/Game/Inventory/Items/Blueprints/Items/BaseItem_BP.BaseItem_BP_C|GetItemProps _asbase_item_bp))) (.Stackable (Utilities|Struct|BreakItem (Variables|/Game/Inventory/Items/Blueprints/Items/BaseItem_BP.BaseItem_BP_C|GetItemProps _asbase_item_bp))) (.Type (Utilities|Struct|BreakItem (Variables|/Game/Inventory/Items/Blueprints/Items/BaseItem_BP.BaseItem_BP_C|GetItemProps _asbase_item_bp))) (.Count (Utilities|Struct|BreakItem (Variables|/Game/Inventory/Items/Blueprints/Items/BaseItem_BP.BaseItem_BP_C|GetItemProps _asbase_item_bp))) (.MaxCount (Utilities|Struct|BreakItem (Variables|/Game/Inventory/Items/Blueprints/Items/BaseItem_BP.BaseItem_BP_C|GetItemProps _asbase_item_bp))) (.Icon (Utilities|Struct|BreakItem (Variables|/Game/Inventory/Items/Blueprints/Items/BaseItem_BP.BaseItem_BP_C|GetItemProps _asbase_item_bp))) (.Class (Utilities|Struct|BreakItem (Variables|/Game/Inventory/Items/Blueprints/Items/BaseItem_BP.BaseItem_BP_C|GetItemProps _asbase_item_bp))))))
          (Utilities|Time|ClearandInvalidateTimerbyHandle (Variables|Burning|GetBurning_TH))
          (Components|Activation|SetActive (Variables|Default|GetParticleSystem) false false)
          (CallFunction|ResetIgniteDoOnce))))))

(event Custom|RotateHUD
  (bind _returnvalue (Game|GetPlayerCharacter 0))
  (bind _furnace_umg (Variables|Default|GetFurnace_UMG))
  ;[1 1 1] Rotate HUD to players rotation
  (Utilities|IsValid _returnvalue
    (:Is%20Valid
      (Transformation|SetWorldRotation _furnace_umg (Math|Rotator|MakeRotator 0.0 0.0 (.Yaw (Math|Rotator|BreakRotator (Math|Rotator|FindLookatRotation (Transformation|GetWorldLocation _furnace_umg) (Transformation|GetWorldLocation (Variables|/Script/Engine.Character|GetCapsuleComponent _returnvalue)))))) false false)
      (bind _asumg_bw_items_hud (Utilities|Casting|CastToUMG_BW_ItemsHUD (UserInterface|GetUserWidgetObject _furnace_umg)))
      (Variables|/Game/Inventory/HUD/ItemsHUD/UMG_BW_ItemsHUD.UMG_BW_ItemsHUD_C|SetHUD_Fuel _asumg_bw_items_hud (Utilities|Text|ToText(String) (Utilities|String|Append "Fuel: " (Utilities|String|ToString(Integer) (Variables|Fuel|GetFuelFill)) "/20")))
      (Variables|/Game/Inventory/HUD/ItemsHUD/UMG_BW_ItemsHUD.UMG_BW_ItemsHUD_C|SetHUD_Name _asumg_bw_items_hud (Utilities|Text|ToText(String) (.Name (Utilities|Struct|BreakItem (Variables|Default|GetItemProps))))))))

(event Custom|CountDown
  (bind _materialsburning (Variables|Materials|GetMaterialsBurning))
  (bind _materialsburning_2 (Variables|Materials|GetMaterialsBurning))
  ;[1 1 1] CountDown -> When adding fuel or amterial item enables physics for 3 seconds
  (Utilities|FlowControl|Sequence
    (:then_0
      (Utilities|FlowControl|DoOnce false
        (:Completed
          (Utilities|FlowControl|Sequence
            (:then_0
              (for _array_element (Variables|Fuel|GetFuel)
                (Class|UsingItemsInterface|EnablePhysic(Message) _array_element)))
            (:then_1
              (for _array_element_2 _materialsburning
                (if (Utilities|IsValid (.MaterialObject (Utilities|Struct|BreakSTR_BurningItem _array_element_2)))
                  (Class|UsingItemsInterface|EnablePhysic(Message) (.MaterialObject (Utilities|Struct|BreakSTR_BurningItem _array_element_2)))
                  (else
                    (Utilities|Array|RemoveItem _materialsburning _array_element_2)
                    (Variables|Materials|SetMaterialFill (- (Variables|Materials|GetMaterialFill) 1))))))))))
    (:then_1
      (bind _output_get (Variables|Fuel|SetTimer (Math|Interpolation|FInterptoConstant (Variables|Fuel|GetTimer) 0.0 (Variables|Burning|GetTimeTick) 1.0)))
      (if (not (> _output_get 0.0))
        (Utilities|FlowControl|Sequence
          (:then_0
            (for _array_element_3 (Variables|Fuel|GetFuel)
              (Class|UsingItemsInterface|DisablePhysic(Message) _array_element_3)))
          (:then_1
            (for _array_element_4 _materialsburning_2
              (if (Utilities|IsValid (.MaterialObject (Utilities|Struct|BreakSTR_BurningItem _array_element_4)))
                (Class|UsingItemsInterface|DisablePhysic(Message) (.MaterialObject (Utilities|Struct|BreakSTR_BurningItem _array_element_4)))
                (else
                  (Utilities|Array|RemoveItem _materialsburning_2 _array_element_4)
                  (Variables|Materials|SetMaterialFill (- (Variables|Materials|GetMaterialFill) 1))))))
          (:then_2
            (Utilities|Time|ClearandInvalidateTimerbyHandle (Variables|Fuel|GetCountDown_TH)))
          (:then_3
            (CallFunction|ResetPhysicsDoOnce)))))))

(event Custom|ResetPhysicsDoOnce
  (bind _materialsburning (Variables|Materials|GetMaterialsBurning))
  ;[1 1 1] CountDown -> When adding fuel or amterial item enables physics for 3 seconds
  (Utilities|FlowControl|DoOnce false) ; enters at Reset
)

(event Custom|ResetIgniteDoOnce
  (bind _particlesystem (Variables|Default|GetParticleSystem))
  ;[1 1 1] Event Ignite -> When filled with fuel can be ignited with flintLighter
  (Utilities|FlowControl|DoOnce false) ; enters at Reset
)

(event Custom|ResetFireDoOnce
  ;[1 1 1] Event Fire -> When ignited
  (Utilities|FlowControl|DoOnce false) ; enters at Reset
)

(event Custom|ResetElapsingDoOnce
  (bind _fuel (Variables|Fuel|GetFuel))
  ;[1 1 1] Event Fire -> When ignited
  (Utilities|FlowControl|DoOnce false) ; enters at Reset
)

(event EventBeginPlay
  ;[1 1 1] BeginPlay Event -> Start timer to RotateHUD
  (|CallParentFunction)
  (Variables|Burning|SetTimeTick 0.05)
  (bind _returnvalue (Utilities|Time|SetTimerbyFunctionName self "RotateHUD" 0.01 true))
  (Variables|Default|SetRotateHUD_TH _returnvalue))

(event EventPutItem
  (params (Class :type Actor%20Class%20Reference))
  ;[1 1 1] Event PutItem -> putting items in furnace (to melt or burn)
  (if (< (Variables|Materials|GetMaterialFill) 5)
    (bind _returnvalue (Game|SpawnActorfromClass Class (Math|Transform|MakeTransform (+ (Transformation|GetActorLocation) "0, 0,100.000000") (Math|Random|RandomRotator false)) "Undefined" 0 0))
    (bind _asbase_item_bp (Utilities|Casting|CastToBaseItem_BP _returnvalue))
    (Variables|/Game/Inventory/Items/Blueprints/Items/BaseItem_BP.BaseItem_BP_C|SetItemProps _asbase_item_bp (Utilities|Struct|MakeItem (.ID (Utilities|Struct|BreakItem (Variables|/Game/Inventory/Items/Blueprints/Items/BaseItem_BP.BaseItem_BP_C|GetItemProps _asbase_item_bp))) (.Name (Utilities|Struct|BreakItem (Variables|/Game/Inventory/Items/Blueprints/Items/BaseItem_BP.BaseItem_BP_C|GetItemProps _asbase_item_bp))) (.Stackable (Utilities|Struct|BreakItem (Variables|/Game/Inventory/Items/Blueprints/Items/BaseItem_BP.BaseItem_BP_C|GetItemProps _asbase_item_bp))) (.Type (Utilities|Struct|BreakItem (Variables|/Game/Inventory/Items/Blueprints/Items/BaseItem_BP.BaseItem_BP_C|GetItemProps _asbase_item_bp))) (.Count (Utilities|Struct|BreakItem (Variables|/Game/Inventory/Items/Blueprints/Items/BaseItem_BP.BaseItem_BP_C|GetItemProps _asbase_item_bp))) (.MaxCount (Utilities|Struct|BreakItem (Variables|/Game/Inventory/Items/Blueprints/Items/BaseItem_BP.BaseItem_BP_C|GetItemProps _asbase_item_bp))) (.Icon (Utilities|Struct|BreakItem (Variables|/Game/Inventory/Items/Blueprints/Items/BaseItem_BP.BaseItem_BP_C|GetItemProps _asbase_item_bp))) (.Class (Utilities|Struct|BreakItem (Variables|/Game/Inventory/Items/Blueprints/Items/BaseItem_BP.BaseItem_BP_C|GetItemProps _asbase_item_bp))) false))
    (Variables|Fuel|SetTimer 3.0)
    (if (Utilities|Time|IsTimerActivebyHandle (Variables|Fuel|GetCountDown_TH))
      (CallFunction|ResetPhysicsDoOnce)
      (Utilities|Time|ClearandInvalidateTimerbyHandle (Variables|Fuel|GetCountDown_TH)))
    (bind _returnvalue_2 (Utilities|Time|SetTimerbyFunctionName self "CountDown" (Variables|Burning|GetTimeTick) true))
    (Variables|Fuel|SetCountDown_TH _returnvalue_2)
    (for _array_element (Variables|Materials|GetMaterialItems)
      (if (== (.MaterialObject (Utilities|Struct|BreakSTR_MaterialItem _array_element)) Class)
        (Utilities|Array|Add (Variables|Materials|GetMaterialsBurning) (Utilities|Struct|MakeSTR_BurningItem _returnvalue (.RemeltItem (Utilities|Struct|BreakSTR_MaterialItem _array_element)) false))
        (Variables|Materials|SetMaterialFill (+ (Variables|Materials|GetMaterialFill) (.MaterialCapacity (Utilities|Struct|BreakSTR_MaterialItem _array_element))))))))

(event EventAddFuel
  (params (FuelClass :type Actor%20Class%20Reference))
  ;[1 1 1] Event AddFuel -> Adding fuel items (for burning)
  (if (< (Variables|Fuel|GetFuelFill) 20)
    (CallFunction|ResetFireDoOnce)
    (bind _returnvalue (Game|SpawnActorfromClass FuelClass (Math|Transform|MakeTransform (+ (Transformation|GetActorLocation) "0, 0,100.000000") (Math|Random|RandomRotator false)) "Undefined" 0 0))
    (bind _asbase_item_bp (Utilities|Casting|CastToBaseItem_BP _returnvalue))
    (Variables|/Game/Inventory/Items/Blueprints/Items/BaseItem_BP.BaseItem_BP_C|SetItemProps _asbase_item_bp (Utilities|Struct|MakeItem (.ID (Utilities|Struct|BreakItem (Variables|/Game/Inventory/Items/Blueprints/Items/BaseItem_BP.BaseItem_BP_C|GetItemProps _asbase_item_bp))) (.Name (Utilities|Struct|BreakItem (Variables|/Game/Inventory/Items/Blueprints/Items/BaseItem_BP.BaseItem_BP_C|GetItemProps _asbase_item_bp))) (.Stackable (Utilities|Struct|BreakItem (Variables|/Game/Inventory/Items/Blueprints/Items/BaseItem_BP.BaseItem_BP_C|GetItemProps _asbase_item_bp))) (.Type (Utilities|Struct|BreakItem (Variables|/Game/Inventory/Items/Blueprints/Items/BaseItem_BP.BaseItem_BP_C|GetItemProps _asbase_item_bp))) (.Count (Utilities|Struct|BreakItem (Variables|/Game/Inventory/Items/Blueprints/Items/BaseItem_BP.BaseItem_BP_C|GetItemProps _asbase_item_bp))) (.MaxCount (Utilities|Struct|BreakItem (Variables|/Game/Inventory/Items/Blueprints/Items/BaseItem_BP.BaseItem_BP_C|GetItemProps _asbase_item_bp))) (.Icon (Utilities|Struct|BreakItem (Variables|/Game/Inventory/Items/Blueprints/Items/BaseItem_BP.BaseItem_BP_C|GetItemProps _asbase_item_bp))) (.Class (Utilities|Struct|BreakItem (Variables|/Game/Inventory/Items/Blueprints/Items/BaseItem_BP.BaseItem_BP_C|GetItemProps _asbase_item_bp))) false))
    (Variables|Fuel|SetTimer 3.0)
    (if (Utilities|Time|IsTimerActivebyHandle (Variables|Fuel|GetCountDown_TH))
      (CallFunction|ResetPhysicsDoOnce)
      (Utilities|Time|ClearandInvalidateTimerbyHandle (Variables|Fuel|GetCountDown_TH)))
    (bind _returnvalue_2 (Utilities|Time|SetTimerbyFunctionName self "CountDown" (Variables|Burning|GetTimeTick) true))
    (Variables|Fuel|SetCountDown_TH _returnvalue_2)
    (Utilities|Array|Add (Variables|Fuel|GetFuel) _returnvalue)
    (for _array_element (Variables|Fuel|GetFuelItems)
      (if (== (.FuelObject (Utilities|Struct|BreakSTR_FuelItem _array_element)) FuelClass)
        (Variables|Fuel|SetFuelFill (+ (Variables|Fuel|GetFuelFill) (.FuelCapacity (Utilities|Struct|BreakSTR_FuelItem _array_element))))
        (Variables|Burning|SetBurnTime (+ (Variables|Burning|GetBurnTime) (.BurnTime (Utilities|Struct|BreakSTR_FuelItem _array_element))))))))

(event EventIgnite
  (bind _particlesystem (Variables|Default|GetParticleSystem))
  ;[1 1 1] Event Ignite -> When filled with fuel can be ignited with flintLighter
  (if (and (> (Variables|Fuel|GetFuelFill) 0) (> (Variables|Burning|GetBurnTime) 0.0))
    (Utilities|FlowControl|DoOnce false
      (:Completed
        (CallFunction|ResetFireDoOnce)
        (CallFunction|ResetElapsingDoOnce)
        (bind _returnvalue (Utilities|Time|SetTimerbyFunctionName self "Fire" (Variables|Burning|GetTimeTick) true))
        (Variables|Burning|SetBurning_TH _returnvalue)
        (Variables|Burning|SetElapsed 0.0)
        (bind _output_get (Variables|Burning|SetScale 0.0))
        (Transformation|SetRelativeScale3D _particlesystem (Math|Vector|MakeVector _output_get _output_get _output_get))
        (Components|Activation|SetActive _particlesystem true false)))))

(fn ConstructionScript
  (|CallParentFunction))