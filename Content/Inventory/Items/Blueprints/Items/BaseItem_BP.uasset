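; Base item Blueprint for the inventory system, holding an item's properties in ItemProps.
; The construction script fills ItemProps from the ItemsDataTable row matching RowName, printing a message if the row is missing.
; SetItemProps replaces those properties directly.
; Use only prints the row name as a debug message, and ChangeRoastedItem is an empty stub.
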(event EventBeginPlay)

(event Collision|EventActorBeginOverlap
  (params (OtherActor :type Actor%20Object%20Reference)))

(event EventTick
  (params (DeltaSeconds :type Float%20%28single-precision%29)))

(event EventUse
  (Development|PrintString (Utilities|String|Append "Using " (Utilities|String|ToString(Name) (Variables|Default|GetRowName)))))

(fn ConstructionScript
  (bind _rowname (Variables|Default|GetRowName))
  (bind _returnvalue (Utilities|GetDataTableRow "/Game/Inventory/Items/Blueprints/ItemsDataTable.ItemsDataTable" _rowname)
    (:then
      (Variables|Default|SetItemProps _returnvalue))
    (:RowNotFound
      (Development|PrintString (Utilities|String|Append (Utilities|String|ToString(Name) _rowname) "   " "Item not found in database")))))

(fn SetItemProps
  (params (GivenItem :type Item%20Structure))
  (Variables|Default|SetItemProps GivenItem))

(fn ChangeRoastedItem)