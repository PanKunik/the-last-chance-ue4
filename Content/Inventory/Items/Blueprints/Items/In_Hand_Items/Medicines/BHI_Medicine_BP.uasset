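; In-hand medicine item Blueprint that handles consuming a medicine and offers cures for bleeding, sunburn and food poisoning.
; Use decrements the item count, notifies the instigator through a message call and plays a 2D sound.
; Each cure function forwards a message to the instigator, but none is called within this Blueprint.
; A leftover "Treating" debug print is disconnected, and the other events are disabled stubs.
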(event EventBeginPlay
  (|CallParentFunction) ; This node is disabled and will not be called.\nDrag off pins to build functionality.
)

(event Collision|EventActorBeginOverlap
  (params (OtherActor :type Actor%20Object%20Reference))
  (|CallParentFunction OtherActor) ; This node is disabled and will not be called.\nDrag off pins to build functionality.
)

(event EventTick
  (params (DeltaSeconds :type Float%20%28single-precision%29))
  (|CallParentFunction DeltaSeconds) ; This node is disabled and will not be called.\nDrag off pins to build functionality.
)

(event EventUse
  (CallFunction|RemoveOneCount)
  (Class|RemoveItem|RemoveOneItemCount(Message) (Game|GetInstigator))
  (Audio|PlaySound2D (Variables|Default|GetSound) 0.5 1.0 0.0 0 0))

(fn ConstructionScript
  (|CallParentFunction))

(fn CureforBleeding
  (Class|PlayerStatistics|CureBleeding(Message) (Game|GetInstigator)))

(fn CureforSunburn
  (Class|PlayerStatistics|CureSunBurn(Message) (Game|GetInstigator)))

(fn CureforFoodPoisoning
  (Class|PlayerStatistics|CureFoodPoisoning(Message) (Game|GetInstigator)))