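; In-hand food item Blueprint that the holder consumes to restore hydration and nutrition.
; On Use it decrements its own item count, or clears the item properties if the count is already zero.
; It then sends its Thirst and Food values to the Instigator as hydration and nutrition messages, followed by a message to remove one item count.
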(event EventBeginPlay
  (|CallParentFunction) ; This node is disabled and will not be called.\nDrag off pins to build functionality.
)

(event Collision|EventActorBeginOverlap
  (params (OtherActor :type Actor%20Object%20Reference))
  (|CallParentFunction OtherActor) ; This node is disabled and will not be called.\nDrag off pins to build functionality.
)

(event EventTick
  (params (DeltaSeconds :type Float%20%28single-precision%29))
  (|CallParentFunction DeltaSeconds) ; This node is disabled and will not be called.\nDrag off pins to build functionality.
)

(event EventUse
  (CallFunction|RemoveOneCount)
  (CallFunction|Eat (Variables|Default|GetThirst) (Variables|Default|GetFood))
  (Class|RemoveItem|RemoveOneItemCount(Message) (Game|GetInstigator)))

(fn ConstructionScript
  (|CallParentFunction))

(fn Eat
  (params (Thirst :type Float%20%28single-precision%29) (Food :type Float%20%28single-precision%29))
  (bind _returnvalue (Game|GetInstigator))
  (Class|PlayerStatistics|Hydration(Message) _returnvalue Thirst)
  (Class|PlayerStatistics|Nutrition(Message) _returnvalue Food))

(fn RemoveOneCount
  (bind _itemprops (Variables|Default|GetItemProps))
  (bind (_id _name _stackable _type _count _maxcount _icon _class _ispickupable) (Utilities|Struct|BreakItem _itemprops))
  (if (> _count 0)
    (CallFunction|SetItemProps (Utilities|Struct|MakeItem _id _name _stackable _type (- _count 1) _maxcount _icon _class _ispickupable))
    (else
      (CallFunction|SetItemProps (Utilities|Struct|MakeItem)))))