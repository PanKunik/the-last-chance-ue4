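; In-hand inventory item for a wooden bowl of fruit soup that the player eats, leaving an empty bowl.
; On Use it removes one count, calls Eat with its Thirst and Food values, and messages the instigator to remove one item.
; It then looks up the WoodenBowl data table row, adds it to the first player's FirstPersonCharacter inventory and refreshes the inventory HUD.
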(event EventBeginPlay
  (|CallParentFunction) ; This node is disabled and will not be called.\nDrag off pins to build functionality.
)

(event Collision|EventActorBeginOverlap
  (params (OtherActor :type Actor%20Object%20Reference))
  (|CallParentFunction OtherActor) ; This node is disabled and will not be called.\nDrag off pins to build functionality.
)

(event EventTick
  (params (DeltaSeconds :type Float%20%28single-precision%29))
  (|CallParentFunction DeltaSeconds) ; This node is disabled and will not be called.\nDrag off pins to build functionality.
)

(event EventUse
  (CallFunction|RemoveOneCount)
  (CallFunction|Eat (Variables|Default|GetThirst) (Variables|Default|GetFood))
  (Class|RemoveItem|RemoveOneItemCount(Message) (Game|GetInstigator))
  (bind _returnvalue (Utilities|GetDataTableRow "/Game/Inventory/Items/Blueprints/ItemsDataTable.ItemsDataTable" "WoodenBowl")
    (:then
      (bind _asfirst_person_character (Utilities|Casting|CastToFirstPersonCharacter (Game|GetPlayerCharacter 0)))
      (Class|InventoryActionsInterface|AddItemtoInventory(Message) _asfirst_person_character _returnvalue)
      (Default|UpdateInventoryHUD _asfirst_person_character))))

(fn ConstructionScript
  (|CallParentFunction))