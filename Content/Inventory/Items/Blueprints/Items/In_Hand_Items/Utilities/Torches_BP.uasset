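; Torch item that can be ignited, burns down over a limited time and destroys itself, with a randomly picked mesh variant.
; Holding the flint lighter reveals an Ignite prompt; Ignite makes the torch non-pickupable and swaps in a burn-time HUD, refreshed by RotateHUD.
; A looping timer, instead of Tick, drains burn time and interpolates the fire particle's scale up, then down near expiry.
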(event Custom|Fire
  (if (> (Variables|Default|GetBurnTime) 0.0)
    (if (> (Variables|Default|GetBurnTime) (Variables|Default|GetExpirationTime))
      (Transformation|SetWorldScale3D (Variables|Default|GetFire_PS) (Math|Vector|MakeVector (Math|Interpolation|FInterptoConstant (Variables|Default|GetScale) 1.0 (Variables|Default|GetTimeTick) 0.375) (Math|Interpolation|FInterptoConstant (Variables|Default|GetScale) 1.0 (Variables|Default|GetTimeTick) 0.375) (Math|Interpolation|FInterptoConstant (Variables|Default|GetScale) 1.0 (Variables|Default|GetTimeTick) 0.375)))
      (Variables|Default|SetScale (Math|Interpolation|FInterptoConstant (Variables|Default|GetScale) 1.0 (Variables|Default|GetTimeTick) 0.375))
      (Variables|Default|SetBurnTime (Math|Interpolation|FInterptoConstant (Variables|Default|GetBurnTime) 0.0 (Variables|Default|GetTimeTick) 1.0))
      (else
        (Transformation|SetWorldScale3D (Variables|Default|GetFire_PS) (Math|Vector|MakeVector (Math|Interpolation|FInterptoConstant (Variables|Default|GetScale) 0.0 (Variables|Default|GetTimeTick) 0.375) (Math|Interpolation|FInterptoConstant (Variables|Default|GetScale) 0.0 (Variables|Default|GetTimeTick) 0.375) (Math|Interpolation|FInterptoConstant (Variables|Default|GetScale) 0.0 (Variables|Default|GetTimeTick) 0.375)))
        (Variables|Default|SetScale (Math|Interpolation|FInterptoConstant (Variables|Default|GetScale) 0.0 (Variables|Default|GetTimeTick) 0.375))
        (Variables|Default|SetBurnTime (Math|Interpolation|FInterptoConstant (Variables|Default|GetBurnTime) 0.0 (Variables|Default|GetTimeTick) 1.0))))
    (else
      (Utilities|Time|ClearandInvalidateTimerbyHandle (Variables|Default|GetBurning_TH))
      (Components|Activation|SetActive (Variables|Default|GetFire_PS) false false)
      (Variables|Default|SetScale 0.0)
      (Actor|DestroyActor))))

(event EventBeginPlay
  (|CallParentFunction)
  (Variables|Default|SetScale 0.0)
  (Components|Activation|SetActive (Variables|Default|GetFire_PS) false true)
  (bind _output_get (Variables|Default|SetBurnTime 6e+02))
  (Variables|Default|SetMaxBurnTime _output_get)
  (Variables|Default|SetExpirationTime 15.0)
  (Variables|Default|SetTimeTick 0.05)
  (if (Utilities|String|Contains (Utilities|GetObjectName (Variables|/Script/Engine.StaticMeshComponent|GetStaticMesh (Variables|Default|GetItemMesh))) "002")
    (Transformation|AddLocalOffset (Variables|Default|GetFire_PS) "0,-1.000000,-5.000000" false false)))

(event Collision|EventActorBeginOverlap
  (params (OtherActor :type Actor%20Object%20Reference))
  (|CallParentFunction OtherActor) ; This node is disabled and will not be called.\nDrag off pins to build functionality.
)

(event EventTick
  (params (DeltaSeconds :type Float%20%28single-precision%29))
  (|CallParentFunction DeltaSeconds) ; This node is disabled and will not be called.\nDrag off pins to build functionality.
)

(event EventIgnite
  (bind _itemprops (Variables|Default|GetItemProps))
  (bind (_id _name _stackable _type _count _maxcount _icon _class) (Utilities|Struct|BreakItem _itemprops))
  (if (> (Variables|Default|GetBurnTime) 0.0)
    (if (not (Utilities|Time|IsTimerActivebyHandle (Variables|Default|GetBurning_TH)))
      (bind _returnvalue (Utilities|Time|SetTimerbyFunctionName self "Fire" (Variables|Default|GetTimeTick) true))
      (Variables|Default|SetBurning_TH _returnvalue)
      (Components|Activation|SetActive (Variables|Default|GetFire_PS) true true)
      (CallFunction|SetItemProps (Utilities|Struct|MakeItem _id _name _stackable _type _count _maxcount _icon _class false))
      (bind _returnvalue_2 (UserInterface|CreateWidget "/Game/Inventory/HUD/ItemsHUD/UMG_BW_TorchHUD.UMG_BW_TorchHUD_C" (Game|GetPlayerController 0)))
      (UserInterface|SetWidget (Variables|Default|GetWidget) _returnvalue_2)
      (Variables|/Game/Inventory/HUD/ItemsHUD/UMG_BW_TorchHUD.UMG_BW_TorchHUD_C|SetHUD_Burntime _returnvalue_2 (Utilities|Text|ToText(String) (Utilities|String|Append (Utilities|String|ToString(Integer) (Math|Float|Round (Variables|Default|GetBurnTime))) " s")))
      (bind _returnvalue_3 (Utilities|GetDataTableRow "/Game/Inventory/Items/Blueprints/ItemsDataTable.ItemsDataTable" "Torches")
        (:then
          (Variables|/Game/Inventory/HUD/ItemsHUD/UMG_BW_TorchHUD.UMG_BW_TorchHUD_C|SetHUD_ItemName _returnvalue_2 (Utilities|Text|ToText(String) (.Name (Utilities|Struct|BreakItem _returnvalue_3))))
          (Variables|/Game/Inventory/HUD/ItemsHUD/UMG_BW_TorchHUD.UMG_BW_TorchHUD_C|SetHUD_ProgressBarValue _returnvalue_2 (/ (Variables|Default|GetBurnTime) (Variables|Default|GetMaxBurnTime))))))))

(event EventRotateHUD
  (|CallParentFunction)
  (bind _asumg_bw_torch_hud (Utilities|Casting|CastToUMG_BW_TorchHUD (UserInterface|GetUserWidgetObject (Variables|Default|GetWidget))))
  (Variables|/Game/Inventory/HUD/ItemsHUD/UMG_BW_TorchHUD.UMG_BW_TorchHUD_C|SetHUD_ProgressBarValue _asumg_bw_torch_hud (/ (Variables|Default|GetBurnTime) (Variables|Default|GetMaxBurnTime)))
  (Variables|/Game/Inventory/HUD/ItemsHUD/UMG_BW_TorchHUD.UMG_BW_TorchHUD_C|SetHUD_Burntime _asumg_bw_torch_hud (Utilities|Text|ToText(String) (Utilities|String|Append (Utilities|String|ToString(Integer) (Math|Float|Round (Variables|Default|GetBurnTime))) " s"))))

(event EventCheckActiveItem
  (bind _widget (Variables|Default|GetWidget))
  (bind _returnvalue (UserInterface|GetUserWidgetObject _widget))
  (bind _asfirst_person_character (Utilities|Casting|CastToFirstPersonCharacter (Game|GetPlayerCharacter 0)))
  (if (== (.Class (Utilities|Struct|BreakItem (Variables|/Game/FirstPersonBP/Blueprints/FirstPersonCharacter.FirstPersonCharacter_C|GetActiveItem _asfirst_person_character))) "/Game/Inventory/Items/Blueprints/Items/In_Hand_Items/Utilities/FlintLighterItem_BP.FlintLighterItem_BP_C")
    (bind _asumg_bw_item_hud (Utilities|Casting|CastToUMG_BW_ItemHUD _returnvalue))
    (Variables|/Game/Inventory/HUD/ItemsHUD/UMG_BW_ItemHUD.UMG_BW_ItemHUD_C|SetHUD_KeyDetails _asumg_bw_item_hud "Ignite")
    (Variables|/Game/Inventory/HUD/ItemsHUD/UMG_BW_ItemHUD.UMG_BW_ItemHUD_C|SetHUD_KeyVisibility _asumg_bw_item_hud "Visible")
    (else
      (bind _asumg_bw_item_hud_2 (Utilities|Casting|CastToUMG_BW_ItemHUD _returnvalue))
      (Variables|/Game/Inventory/HUD/ItemsHUD/UMG_BW_ItemHUD.UMG_BW_ItemHUD_C|SetHUD_KeyVisibility _asumg_bw_item_hud_2 "Hidden"))))

(fn ConstructionScript
  (|CallParentFunction)
  (Components|StaticMesh|SetStaticMesh (Variables|Default|GetItemMesh) (Utilities|Array|Get(acopy) (Variables|Default|GetMeshes) (Math|Random|RandomIntegerinRange 0 1))))