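; CampfireCoal_BP is a campfire coal Blueprint filed under the inventory's resource items.
; On BeginPlay it hides ItemMesh and its other static mesh components without propagating to children, then adds an entry to the FuelItems array.
; The construction script only calls the parent's, and no logic here makes the meshes visible again or consumes the fuel.
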(event EventBeginPlay
  (Rendering|SetVisibility (Variables|Default|GetItemMesh) false false)
  (Utilities|Array|Add (Variables|Default|GetFuelItems) 0))

(event Collision|EventActorBeginOverlap
  (params (OtherActor :type Actor%20Object%20Reference)))

(event EventTick
  (params (DeltaSeconds :type Float%20%28single-precision%29)))

(fn ConstructionScript
  (|CallParentFunction))