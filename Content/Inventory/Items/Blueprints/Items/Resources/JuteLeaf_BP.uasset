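; JuteLeaf_BP is an inventory resource item for a jute leaf, built on a parent item class that handles BeginPlay and construction.
; DisablePhysic and EnablePhysic events toggle physics simulation on its ItemMesh.
; The Use event is empty.
; An unconnected camera line trace would send AddFuelMessage with the item's class to actors implementing UsingItemsInterface, but never runs.
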(event EventBeginPlay
  (|CallParentFunction))

(event Collision|EventActorBeginOverlap
  (params (OtherActor :type Actor%20Object%20Reference)))

(event EventTick
  (params (DeltaSeconds :type Float%20%28single-precision%29)))

(event EventUse)

(event EventDisablePhysic
  (Physics|SetSimulatePhysics (Variables|Default|GetItemMesh) false))

(event EventEnablePhysic
  (Physics|SetSimulatePhysics (Variables|Default|GetItemMesh) true))

(fn ConstructionScript
  (|CallParentFunction))