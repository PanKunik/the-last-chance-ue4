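; Wood resource inventory item that can be used as fuel on objects in the world.
; On Use, it line traces from the player camera up to PickupDistance and sends its class through AddFuelMessage to a hit actor implementing UsingItemsInterface.
; The construction script runs the parent's, then picks a random mesh from WoodMeshes for visual variety.
; EnablePhysic and DisablePhysic events toggle physics simulation on the item mesh.
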(event EventBeginPlay)

(event Collision|EventActorBeginOverlap
  (params (OtherActor :type Actor%20Object%20Reference)))

(event EventUse
  (bind _returnvalue (Game|GetPlayerCameraManager 0))
  (bind _returnvalue_2 (Transformation|GetActorLocation _returnvalue))
  (bind _outhit (Collision|LineTraceByChannel _returnvalue_2 (+ _returnvalue_2 (* (Transformation|GetActorForwardVector _returnvalue) (Variables|Default|GetPickupDistance))) "TraceTypeQuery1" false 0 "None" true "(R=1.000000,G=0.000000,B=0.000000,A=1.000000)" "(R=0.000000,G=1.000000,B=0.000000,A=1.000000)" 5e+02))
  (if (Utilities|DoesObjectImplementInterface (.HitActor (Collision|BreakHitResult _outhit)) "/Game/Inventory/Items/Blueprints/Items/Utilities/UsingItemsInterface.UsingItemsInterface_C")
    (Class|UsingItemsInterface|AddFuel(Message) (.HitActor (Collision|BreakHitResult _outhit)) (Utilities|GetClass self))))

(event EventEnablePhysic
  (Physics|SetSimulatePhysics (Variables|Default|GetItemMesh) true))

(event EventDisablePhysic
  (Physics|SetSimulatePhysics (Variables|Default|GetItemMesh) false))

(fn ConstructionScript
  (|CallParentFunction)
  (Components|StaticMesh|SetStaticMesh (Variables|Default|GetItemMesh) (Utilities|Array|Get(acopy) (Variables|Default|GetWoodMeshes) (Math|Random|RandomIntegerinRange 0 3))))