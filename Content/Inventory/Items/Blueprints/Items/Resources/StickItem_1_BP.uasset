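; Stick resource item that can be offered as fuel to objects in the world.
; On UseF, it box-traces forward from the player camera and sends its class through AddFuelMessage to a hit actor implementing UsingItemsInterface.
; The construction script picks a random stick mesh for variety.
; EnablePhysic and DisablePhysic events toggle physics simulation on the item mesh.
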(event EventBeginPlay
  (|CallParentFunction) ; This node is disabled and will not be called.\nDrag off pins to build functionality.
)

(event Collision|EventActorBeginOverlap
  (params (OtherActor :type Actor%20Object%20Reference))
  (|CallParentFunction OtherActor) ; This node is disabled and will not be called.\nDrag off pins to build functionality.
)

(event EventTick
  (params (DeltaSeconds :type Float%20%28single-precision%29))
  (|CallParentFunction DeltaSeconds) ; This node is disabled and will not be called.\nDrag off pins to build functionality.
)

(event EventEnablePhysic
  (Physics|SetSimulatePhysics (Variables|Default|GetItemMesh) true))

(event EventDisablePhysic
  (Physics|SetSimulatePhysics (Variables|Default|GetItemMesh) false))

(event EventUseF
  (bind _returnvalue (Game|GetPlayerCameraManager 0))
  (bind _rootcomponent (Variables|/Script/Engine.Actor|GetRootComponent _returnvalue))
  (bind _returnvalue_2 (Transformation|GetWorldLocation _rootcomponent))
  (bind (_outhit _returnvalue_3) (Class|KismetSystemLibrary|BoxTraceSingleforObjects _returnvalue_2 (+ _returnvalue_2 (* (Math|Vector|GetForwardVector (Variables|/Script/Engine.Actor|GetRootComponent (Game|GetPlayerCameraManager 0))) (Variables|Default|GetUseDistance))) "10.000000,10.000000,10.000000" "0, 0, 0" (Utilities|Array|MakeArray "ObjectTypeQuery8") false 0 "None" true))
  (if _returnvalue_3
    (if (Utilities|DoesObjectImplementInterface (.HitActor (Collision|BreakHitResult _outhit)) "/Game/Inventory/Items/Blueprints/Items/Utilities/UsingItemsInterface.UsingItemsInterface_C")
      (Class|UsingItemsInterface|AddFuel(Message) (.HitActor (Collision|BreakHitResult _outhit)) (Utilities|GetClass self)))))

(fn ConstructionScript
  (|CallParentFunction)
  (Components|StaticMesh|SetStaticMesh (Variables|Default|GetItemMesh) (Utilities|Array|Get(acopy) (Variables|Default|GetStickMeshes) (Math|Random|RandomIntegerinRange 0 2))))