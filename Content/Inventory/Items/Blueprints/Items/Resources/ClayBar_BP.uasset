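; ClayBar_BP is a clay bar resource item that can be placed into world actors and turned into a burned variant.
; Use line traces forward from the player camera and passes the item's class through PutItemMessage to a hit actor implementing UsingItemsInterface.
; Separate events toggle mesh physics, while ChangeBurnedItem swaps mesh, material and item properties to the BurnedItem data, forcing it to be non-pickupable.
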(event EventBeginPlay
  (|CallParentFunction) ; This node is disabled and will not be called.\nDrag off pins to build functionality.
)

(event Collision|EventActorBeginOverlap
  (params (OtherActor :type Actor%20Object%20Reference))
  (|CallParentFunction OtherActor) ; This node is disabled and will not be called.\nDrag off pins to build functionality.
)

(event EventChangeBurnedItem
  (bind _burneditem (Variables|Default|GetBurnedItem))
  (bind _itemmesh (Variables|Default|GetItemMesh))
  (bind (_staticmesh _material _itemvalues) (Utilities|Struct|BreakSTR_ChangedItemOnBurning _burneditem))
  (bind (_id _name _stackable _type _count _maxcount _icon _class) (Utilities|Struct|BreakItem _itemvalues))
  (Components|StaticMesh|SetStaticMesh _itemmesh _staticmesh)
  (Rendering|Material|SetMaterial _itemmesh 0 _material)
  (CallFunction|SetItemProps (Utilities|Struct|MakeItem _id _name _stackable _type _count _maxcount _icon _class false)))

(event EventTick
  (params (DeltaSeconds :type Float%20%28single-precision%29))
  (|CallParentFunction DeltaSeconds) ; This node is disabled and will not be called.\nDrag off pins to build functionality.
)

(event EventUse
  (bind _returnvalue (Game|GetPlayerCameraManager 0))
  (bind _returnvalue_2 (Transformation|GetActorLocation _returnvalue))
  (bind _outhit (Collision|LineTraceByChannel _returnvalue_2 (+ _returnvalue_2 (* (Transformation|GetActorForwardVector _returnvalue) (Variables|Default|GetUseDistance))) "TraceTypeQuery1" false 0 "None" true "(R=1.000000,G=0.000000,B=0.000000,A=1.000000)" "(R=0.000000,G=1.000000,B=0.000000,A=1.000000)" 5e+02))
  (if (Utilities|DoesObjectImplementInterface (.HitActor (Collision|BreakHitResult _outhit)) "/Game/Inventory/Items/Blueprints/Items/Utilities/UsingItemsInterface.UsingItemsInterface_C")
    (Class|UsingItemsInterface|PutItem(Message) (.HitActor (Collision|BreakHitResult _outhit)) (Utilities|GetClass self))))

(event EventDisablePhysic
  (Physics|SetSimulatePhysics (Variables|Default|GetItemMesh) false))

(event EventEnablePhysic
  (Physics|SetSimulatePhysics (Variables|Default|GetItemMesh) true))

(fn ConstructionScript
  (|CallParentFunction))